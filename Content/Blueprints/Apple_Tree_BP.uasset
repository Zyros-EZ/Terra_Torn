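; Harvestable apple tree that gives the player apples when interacted with and regrows them later.
; A sphere overlap sets the character's NextToInteractable flag.
; Interact hides six apple components, spawns Apple_BP actors in their place, then after delays destroys every Apple_BP in the world, calls GivePlayerApples and restores the components.
; IsHarvestable gates harvesting, while the character's DoesTakeEnergy is switched off on drop and on at start and regrowth.
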(event `self.ReceiveBeginPlay`
  (`KismetSystemLibrary.Delay` 1.0)
  (bind _returnvalue (`GameplayStatics.GetActorOfClass` "/Game/ThirdPerson/Blueprints/BP_ThirdPersonCharacter.BP_ThirdPersonCharacter_C"))
  (set `/Game/ThirdPerson/Blueprints/BP_ThirdPersonCharacter.DoesTakeEnergy` true _returnvalue))

(event `/Game/Blueprints/Interact_BPI.Interact`
  (params (Character :type "/Game/ThirdPerson/Blueprints/BP_ThirdPersonCharacter Object Reference"))
  ;[1 1 1] Drop Apples - Give Player Apples
  (if (`self.IsHarvestable`)
    (`self.DropApples`)
    (`KismetSystemLibrary.Delay` 2.0)
    (`self.DestroyApples`)
    (`/Engine/EditorBlueprintResources/StandardMacros.IsValid` Character
      (:`Is Valid`
        (`/Game/ThirdPerson/Blueprints/BP_ThirdPersonCharacter.GivePlayerApples` Character self)
        (`KismetSystemLibrary.Delay` 10.0)
        (`self.RegrowApples`)))))

(event `self.Sphere.OnComponentBeginOverlap`
  (params (OverlappedComponent :type "PrimitiveComponent Object Reference") (OtherActor :type "Actor Object Reference") (OtherComp :type "PrimitiveComponent Object Reference") (OtherBodyIndex :type Integer) (bFromSweep :type Boolean) (SweepResult :type "HitResult Structure (by ref)"))
  ;[1 1 1] Detect Player In Range
  (bind _asbp_third_person_character (cast `/Game/ThirdPerson/Blueprints/BP_ThirdPersonCharacter` OtherActor))
  (set `/Game/ThirdPerson/Blueprints/BP_ThirdPersonCharacter.NextToInteractable` true _asbp_third_person_character))

(event `self.Sphere.OnComponentEndOverlap`
  (params (OverlappedComponent :type "PrimitiveComponent Object Reference") (OtherActor :type "Actor Object Reference") (OtherComp :type "PrimitiveComponent Object Reference") (OtherBodyIndex :type Integer))
  ;[1 1 1] Detect Player In Range
  (bind _asbp_third_person_character (cast `/Game/ThirdPerson/Blueprints/BP_ThirdPersonCharacter` OtherActor))
  (set `/Game/ThirdPerson/Blueprints/BP_ThirdPersonCharacter.NextToInteractable` false _asbp_third_person_character))

(fn `DestroyApples`
  (bind _outactors (`GameplayStatics.GetAllActorsOfClass` "/Game/Blueprints/Apple_BP.Apple_BP_C"))
  (for _array_element _outactors
    (`self.K2_DestroyActor` _array_element)
    (`KismetArrayLibrary.Array_RemoveItem` _outactors)))

(fn `DropApples`
  (for _array_element (`|MakeArray` (`self.Apple`) (`self.Apple1`) (`self.Apple2`) (`self.Apple3`) (`self.Apple4`) (`self.Apple5`))
    (`SceneComponent.SetVisibility` _array_element false false)
    (`|SpawnActorFromClass` "/Game/Blueprints/Apple_BP.Apple_BP_C" (`SceneComponent.K2_GetComponentToWorld` _array_element) "Undefined" "MultiplyWithRoot" null null)
    (set `self.IsHarvestable` false)
    (bind _returnvalue (`GameplayStatics.GetActorOfClass` "/Game/ThirdPerson/Blueprints/BP_ThirdPersonCharacter.BP_ThirdPersonCharacter_C"))
    (set `/Game/ThirdPerson/Blueprints/BP_ThirdPersonCharacter.DoesTakeEnergy` false _returnvalue)))

(fn `RegrowApples`
  (for _array_element (`|MakeArray` (`self.Apple`) (`self.Apple1`) (`self.Apple2`) (`self.Apple3`) (`self.Apple4`) (`self.Apple5`))
    (`SceneComponent.SetVisibility` _array_element true false)
    (set `self.IsHarvestable` true)
    (bind _returnvalue (`GameplayStatics.GetActorOfClass` "/Game/ThirdPerson/Blueprints/BP_ThirdPersonCharacter.BP_ThirdPersonCharacter_C"))
    (set `/Game/ThirdPerson/Blueprints/BP_ThirdPersonCharacter.DoesTakeEnergy` true _returnvalue)))

(fn `UserConstructionScript`)