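; Tier 1 compost bin that turns six apples from the player's inventory into one fertilizer item.
; Interact loads an empty bin and spawns a food compost actor, or hands over ready fertilizer.
; Tick uses CompostTimer and a DoOnce to gate ProduceFertilizer, which swaps the compost actor for a fertilizer actor.
; An overlap sphere flags the player as near an interactable, with energy cost disabled on entry.
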(event `self.ReceiveBeginPlay`)

(event `self.ReceiveTick`
  (params (DeltaSeconds :type "Float (single-precision)"))
  (bind _composttimer (`self.CompostTimer`))
  (if (and (> _composttimer 0.0) (`self.IsLoaded`))
    (goto _label :!via `Reset`)
    (else
      (`/Engine/EditorBlueprintResources/StandardMacros.DoOnce` false :!label _label
        (:`Completed`
          (set `self.CompostTimer` (- _composttimer DeltaSeconds))
          (`self.ProduceFertilizer` (stale `/Game/Blueprints/Interact_BPI.Interact` _returnvalue)))))))

(event `/Game/Blueprints/Interact_BPI.Interact`
  (params (Character :type "/Game/ThirdPerson/Blueprints/BP_Player_Character Object Reference"))
  (`|ExecutionSequence`
    (:`then_0`
      (`self.IsCompostBinFull` Character)
      (if (`self.IsLoaded`)
        (bind _returnvalue (`|SpawnActorFromClass` "/Game/Blueprints/FoodCompost_BP.FoodCompost_BP_C" (`SceneComponent.K2_GetComponentToWorld` (`self.Spawnpoint`)) "Undefined" "MultiplyWithRoot" null null))))
    (:`then_1`
      (`self.GivePlayerFertilizer` Character))))

(event `self.Sphere.OnComponentBeginOverlap`
  (params (OverlappedComponent :type "PrimitiveComponent Object Reference") (OtherActor :type "Actor Object Reference") (OtherComp :type "PrimitiveComponent Object Reference") (OtherBodyIndex :type Integer) (bFromSweep :type Boolean) (SweepResult :type "HitResult Structure (by ref)"))
  ;[1 1 1] Is Player In Range
  (bind _asbp_player_character (cast `/Game/ThirdPerson/Blueprints/BP_Player_Character` OtherActor))
  (set `/Game/ThirdPerson/Blueprints/BP_Player_Character.NextToInteractable` true _asbp_player_character)
  (set `/Game/ThirdPerson/Blueprints/BP_Player_Character.DoesTakeEnergy` false _asbp_player_character))

(event `self.Sphere.OnComponentEndOverlap`
  (params (OverlappedComponent :type "PrimitiveComponent Object Reference") (OtherActor :type "Actor Object Reference") (OtherComp :type "PrimitiveComponent Object Reference") (OtherBodyIndex :type Integer))
  ;[1 1 1] Is Player In Range
  (bind _asbp_player_character (cast `/Game/ThirdPerson/Blueprints/BP_Player_Character` OtherActor))
  (set `/Game/ThirdPerson/Blueprints/BP_Player_Character.NextToInteractable` false _asbp_player_character))

(fn `GivePlayerFertilizer`
  (params (PlayerCharacter :type "/Game/ThirdPerson/Blueprints/BP_Player_Character Object Reference"))
  (if (`self.FertilizerReady`)
    (bind _returnvalue (`|GenericCreateObject` "/Game/Blueprints/Inventory/BP_FertilizerItem.BP_FertilizerItem_C"))
    (`/Game/ThirdPerson/Blueprints/BP_Player_Character.AddToInventory` PlayerCharacter _returnvalue 1)
    (set `self.BinInventoryFertilizer` 0)
    (set `self.FertilizerReady` false)
    (`self.K2_DestroyActor` (`self.FertilizerReference`))
    (set `self.FertilizerReference` null)))

(fn `IsCompostBinFull`
  (params (PlayerCharacter :type "/Game/ThirdPerson/Blueprints/BP_Player_Character Object Reference"))
  (if (<= (`self.BinInventoryFertilizer`) 0)
    (if (>= (`self.BinInventoryFood`) 6)
      (set `self.IsLoaded` true)
      (else
        (bind (_item _num) (`/Game/ThirdPerson/Blueprints/BP_Player_Character.GetItem` PlayerCharacter "/Game/Blueprints/Inventory/BP_AppleItem.BP_AppleItem_C"))
        (if (>= _num 6)
          (bind _result (`/Game/ThirdPerson/Blueprints/BP_Player_Character.RemoveFromInventory` PlayerCharacter _item 6))
          (if _result
            (`GameplayStatics.SpawnSoundAtLocation` "/Game/SFX/Apple_Falls.Apple_Falls" (`SceneComponent.K2_GetComponentLocation` (`self.DefaultSceneRoot`)) (struct) 1.0 1.0 0.0 null null)
            (set `self.BinInventoryFood` 6)
            (set `self.IsLoaded` true)
            (set `self.CompostTimer` (`self.CompostTime`)))
          (else
            (set `self.IsLoaded` false)))))))

(fn `ProduceFertilizer`
  (params (CompostRef :type "Actor Object Reference"))
  (if (`self.IsLoaded`)
    (set `self.BinInventoryFood` 0)
    (`self.K2_DestroyActor` CompostRef)
    (set `self.BinInventoryFertilizer` 1)
    (set `self.FertilizerReady` true)
    (set `self.IsLoaded` false)
    (bind _returnvalue (`|SpawnActorFromClass` "/Game/Blueprints/Fertilizer_BP.Fertilizer_BP_C" (`SceneComponent.K2_GetComponentToWorld` (`self.Spawnpoint`)) "Undefined" "MultiplyWithRoot" null null))
    (set `self.FertilizerReference` _returnvalue)))

(fn `ResetTimer`
  (set `self.CompostTimer` 0.0))

(fn `UserConstructionScript`)