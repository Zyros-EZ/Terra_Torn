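; Parent crop actor that grows from seed through a middle stage to harvestable, then adds an item to the player's inventory and destroys itself.
; Watering sets a target day from the HUD widget's day count and starts a looping timer that calls GrowCrop when that day matches.
; Growth swaps stage meshes, and watering and growth change the overlapped soil tile's material.
; Growth timing uses Kiwi-named variables, zeroed on BeginPlay; Interact is empty.
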(event `self.ReceiveBeginPlay`
  (`self.SetGrowthTimeOfKiwi` 0))

(event `self.ReceiveActorBeginOverlap`
  (params (OtherActor :type "Actor Object Reference"))
  (bind _astillable_soil_bp (cast `/Game/Blueprints/TillableSoil_BP` OtherActor))
  (set `self.Farmtile` _astillable_soil_bp))

(event `/Game/Blueprints/Interact_BPI.Interact`
  (params (`Player Character` :type "/Game/ThirdPerson/Blueprints/BP_Player_Character Object Reference")))

(fn `CheckingGrowth`
  (bind _foundwidgets (`WidgetBlueprintLibrary.GetAllWidgetsOfClass` "/Game/ThirdPerson/HUD/WBP_HUD.WBP_HUD_C"))
  (bind _day (`/Game/ThirdPerson/HUD/WBP_HUD.GetDayInt` _foundwidgets))
  (if (== _day (`self.KiwiGrowthDay`))
    (`self.GrowCrop`)))

(fn `GivePlayerCrop`
  (params (PlayerCharacter :type "/Game/ThirdPerson/Blueprints/BP_Player_Character Object Reference") (ItemID :type "/Game/Blueprints/Items/ItemId Enum" :default "NewEnumerator0") (Amount :type Integer :default 1))
  (returns (HasCrop :type Boolean))
  (if (`self.IsHarvestable`)
    (`/Game/Blueprints/Inventory/Inventory.AddToInventory` (`/Game/ThirdPerson/Blueprints/BP_Player_Character.NewInventory` PlayerCharacter) ItemID Amount)
    (`self.K2_DestroyActor`)
    (return false)
    (else
      (return true))))

(fn `GrowCrop`
  (switch `/Game/Blueprints/Crops/E_CropStage` (`self.CurrentStage`)
    (:`NewEnumerator0`
      (`|ExecutionSequence`
        (:`then_0`
          (`SceneComponent.SetVisibility` (`self.SeedMesh`) false false))
        (:`then_1`
          (`SceneComponent.SetVisibility` (`self.Stage1Mesh`) true false))
        (:`then_2`
          (set `self.CurrentStage` "NewEnumerator1"))
        (:`then_3`
          (set `self.IsWatered` false))
        (:`then_4`
          (`self.SetNewGrowthTime`))
        (:`then_5`
          (`PrimitiveComponent.SetMaterial` (`StaticMeshActor.StaticMeshComponent` (`self.Farmtile`)) 0 "/Game/Materials/M_Dirt.M_Dirt"))
        (:`then_6`
          (`KismetSystemLibrary.K2_ClearAndInvalidateTimerHandle` (`self.GrowthTimerHandle`)))))
    (:`NewEnumerator1`
      (`|ExecutionSequence`
        (:`then_0`
          (`SceneComponent.SetVisibility` (`self.Stage1Mesh`) false false))
        (:`then_1`
          (`SceneComponent.SetVisibility` (`self.HarvestableMesh`) true false))
        (:`then_2`
          (set `self.CurrentStage` "NewEnumerator2"))
        (:`then_3`
          (set `self.IsHarvestable` true))
        (:`then_4`
          (`PrimitiveComponent.SetMaterial` (`StaticMeshActor.StaticMeshComponent` (`self.Farmtile`)) 0 "/Game/Materials/M_Dirt.M_Dirt"))))))

(fn `InteractWith`
  (returns (ObjectiveID :type String))
  (return ""))

(fn `SetGrowthTimeOfKiwi`
  (params (KiwiGrowthTime :type Integer))
  (set `self.SpecificKiwiGrowthTime` KiwiGrowthTime))

(fn `SetNewGrowthTime`
  (bind _foundwidgets (`WidgetBlueprintLibrary.GetAllWidgetsOfClass` "/Game/ThirdPerson/HUD/WBP_HUD.WBP_HUD_C"))
  (bind _day (`/Game/ThirdPerson/HUD/WBP_HUD.GetDayInt` _foundwidgets))
  (set `self.KiwiGrowthDay` (+ _day (`self.SpecificKiwiGrowthTime`))))

(fn `TakePlayerEnergy`
  (params (isHarvestable :type Boolean))
  (returns (HasEnergy :type Boolean))
  (return false))

(fn `UserConstructionScript`)

(fn `WaterPlant`
  (if (not (`self.IsWatered`))
    (`|ExecutionSequence`
      (:`then_0`
        (set `self.IsWatered` true)
        (`KismetSystemLibrary.PrintString` "Watered"))
      (:`then_1`
        (`self.SetNewGrowthTime`))
      (:`then_2`
        (`KismetSystemLibrary.K2_ClearAndInvalidateTimerHandle` (`self.GrowthTimerHandle`))
        (bind _returnvalue (`KismetSystemLibrary.K2_SetTimer` null "CheckingGrowth" 0.5 true))
        (set `self.GrowthTimerHandle` _returnvalue))
      (:`then_3`
        (`PrimitiveComponent.SetMaterial` (`StaticMeshActor.StaticMeshComponent` (`self.Farmtile`)) 0 "/Game/CharacterFiles/CharacterMeshes/Idle/ROBOTFIles/AccentColors.AccentColors")))))