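; PumpkinCrop_BP is a pumpkin crop Blueprint that holds references to three growth-stage actors.
; On BeginPlay, after the parent call, it uses GetActorOfClass for each pumpkin stage class and stores the results in Stage1Crop through Stage3Crop.
; Each lookup returns a single actor found in the world, rather than spawning one.
; It adds no other logic of its own.
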(event `self.ReceiveBeginPlay`
  (`parent.ReceiveBeginPlay`)
  (bind _returnvalue (`GameplayStatics.GetActorOfClass` "/Game/Blueprints/Crops/PumpkinStage1_BP.PumpkinStage1_BP_C"))
  (set `self.Stage1Crop` _returnvalue)
  (bind _returnvalue_2 (`GameplayStatics.GetActorOfClass` "/Game/Blueprints/Crops/PumpkinStage2_BP.PumpkinStage2_BP_C"))
  (set `self.Stage2Crop` _returnvalue_2)
  (bind _returnvalue_3 (`GameplayStatics.GetActorOfClass` "/Game/Blueprints/Crops/PumpkinStage3_BP.PumpkinStage3_BP_C"))
  (set `self.Stage3Crop` _returnvalue_3))

(fn `UserConstructionScript`
  (`parent.UserConstructionScript`))