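; Small kiwi pickup actor that the player collects into their inventory.
; Overlapping its sphere flags the player character as next to an interactable; nothing here clears that flag.
; The Interact event adds one item to the player's NewInventory component through AddSmallKiwiToInv, then destroys the actor.
; InteractWith returns an empty string and TakePlayerEnergy returns false.
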(event `self.Sphere.OnComponentBeginOverlap`
  (params (OverlappedComponent :type "PrimitiveComponent Object Reference") (OtherActor :type "Actor Object Reference") (OtherComp :type "PrimitiveComponent Object Reference") (OtherBodyIndex :type Integer) (bFromSweep :type Boolean) (SweepResult :type "HitResult Structure (by ref)"))
  (bind _asbp_player_character (cast `/Game/ThirdPerson/Blueprints/BP_Player_Character` OtherActor))
  (set `/Game/ThirdPerson/Blueprints/BP_Player_Character.NextToInteractable` true _asbp_player_character))

(event `/Game/Blueprints/Interact_BPI.Interact`
  (params (`Player Character` :type "/Game/ThirdPerson/Blueprints/BP_Player_Character Object Reference"))
  (`self.AddSmallKiwiToInv` `Player Character` 1))

(fn `AddSmallKiwiToInv`
  (params (PlayerCharacter :type "/Game/ThirdPerson/Blueprints/BP_Player_Character Object Reference") (Amount :type Integer))
  (`/Game/Blueprints/Inventory/Inventory.AddToInventory` (`/Game/ThirdPerson/Blueprints/BP_Player_Character.NewInventory` PlayerCharacter) "NewEnumerator0" Amount)
  (`self.K2_DestroyActor`))

(fn `InteractWith`
  (returns (ObjectiveID :type String))
  (return ""))

(fn `TakePlayerEnergy`
  (params (isHarvestable :type Boolean))
  (returns (HasEnergy :type Boolean))
  (return false))

(fn `UserConstructionScript`)