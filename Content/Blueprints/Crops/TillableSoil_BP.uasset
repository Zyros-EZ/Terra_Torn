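; Interactable soil plot for farming that the player fertilizes, then plants with corn.
; The first interaction consumes fertilizer, swaps the mesh to dirt, reports the fertilize objective and spawns a location marker.
; Later interactions consume seed to spawn a CornCrop_BP, then forward to that crop to water it or give it to the player.
; FertilizerCheck and SeedCheck gate each stage through the player's inventory.
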(event `self.ReceiveBeginPlay`)

(event `/Game/Blueprints/Interact_BPI.Interact`
  (params (`Player Character` :type "/Game/ThirdPerson/Blueprints/BP_Player_Character Object Reference"))
  (bind _returnvalue (`SceneComponent.K2_GetComponentLocation` (`self.StaticMeshComponent`)))
  ;[1 1 1] Interaction - Fertilize Soil
  (if (not (`self.IsFertilized`))
    (bind _result (`self.FertilizerCheck` `Player Character`))
    (if _result
      (`GameplayStatics.SpawnSoundAtLocation` "/Game/SFX/Hoe.Hoe" _returnvalue (struct) 1.0 1.0 0.0 null null)
      (`PrimitiveComponent.SetMaterial` (`self.StaticMeshComponent`) 0 "/Game/Materials/M_Dirt.M_Dirt")
      (set `self.IsFertilized` true)
      (set `/Game/ThirdPerson/Blueprints/BP_Player_Character.DoesTakeEnergy` false `Player Character`)
      (bind _output_get (set `self.FertilizeObjectiveQuantity` (+ (`self.FertilizeObjectiveQuantity`) 1)))
      (`/Game/ThirdPerson/Blueprints/BP_Player_Character.OnObjectiveIDCalled` `Player Character` "fertilizesoil" _output_get)
      (`|SpawnActorFromClass` "/Game/Blueprints/QuestSystem/LocationMarker_BP.LocationMarker_BP_C" (`KismetMathLibrary.MakeTransform` _returnvalue (struct) (5.0 5.0 1.0)) "Undefined" "MultiplyWithRoot" null (`self.LocationName`) (`self.ObjectiveID`) null))
    (elif (`self.HasCrop`)
      (`GameplayStatics.GetActorOfClass` "/Game/Blueprints/Crops/ParentCrop_BP.ParentCrop_BP_C")
      (`/Game/Blueprints/Crops/ParentCrop_BP.GivePlayerCrop` (stale _returnvalue_2) `Player Character`)
      (`/Game/Blueprints/Crops/ParentCrop_BP.WaterPlant` (stale _returnvalue_2))
      (else
        (bind _output_get_2 (`self.SeedCheck` `Player Character`))
        (if _output_get_2
          (set `self.HasCrop` true)
          (bind _returnvalue_2 (`|SpawnActorFromClass` "/Game/Blueprints/Crops/CornCrop_BP.CornCrop_BP_C" (`KismetMathLibrary.MakeTransform` _returnvalue) "Undefined" "MultiplyWithRoot" null null))
          (set `/Game/ThirdPerson/Blueprints/BP_Player_Character.DoesTakeEnergy` false `Player Character`)
          (set `self.PlantObjectiveQuantity` (+ (`self.PlantObjectiveQuantity`) 1))
          (`/Game/ThirdPerson/Blueprints/BP_Player_Character.OnObjectiveIDCalled` `Player Character` "" 0))))))

(fn `FertilizerCheck`
  (params (InputPin :type "/Game/ThirdPerson/Blueprints/BP_Player_Character Object Reference"))
  (returns (Result :type Boolean))
  (bind (_item _success) (`/Game/ThirdPerson/Blueprints/BP_Player_Character.GetItem` InputPin "NewEnumerator1"))
  (if _success
    (`/Game/Blueprints/Interact_BPI.TakePlayerEnergy` InputPin true)
    (bind _result (`/Game/ThirdPerson/Blueprints/BP_Player_Character.RemoveFromInventory` (`local.InputPin`) _item 1))
    (return _result)
    (else
      (bind _output_get (set `self.IsFertilized` false))
      (return _output_get))))

(fn `InteractWith`
  (returns (ObjectiveID :type String))
  (return ""))

(fn `SeedCheck`
  (params (Player :type "/Game/ThirdPerson/Blueprints/BP_Player_Character Object Reference"))
  (returns (Output_Get :type Boolean))
  (bind (_item _success) (`/Game/ThirdPerson/Blueprints/BP_Player_Character.GetItem` Player "NewEnumerator0"))
  (if _success
    (bind _result (`/Game/ThirdPerson/Blueprints/BP_Player_Character.RemoveFromInventory` Player _item 1))
    (return _result)
    (else
      (bind _output_get (set `/Game/ThirdPerson/Blueprints/BP_Player_Character.DoesTakeEnergy` false Player))
      (return _output_get))))

(fn `TakePlayerEnergy`
  (params (isHarvestable :type Boolean))
  (returns (HasEnergy :type Boolean))
  (return false))

(fn `UserConstructionScript`)