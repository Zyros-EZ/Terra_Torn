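; Tillable soil plot that the player fertilizes and then uses to open a seed-planting menu.
; Interacting consumes a fertilizer item and energy, swaps the mesh to dirt, reports objective progress and spawns a location marker.
; Once fertilized, interaction adds or removes the seed widget based on UIOpen, while box overlap controls the interact prompt.
; Direct corn planting, watering and harvesting logic remains in the graph but never runs.
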(event `self.ReceiveActorBeginOverlap`
  (params (OtherActor :type "Actor Object Reference")))

(event `self.ReceiveBeginPlay`
  (`|ExecutionSequence`
    (:`then_0`
      (bind _returnvalue (`|CreateWidget` "/Game/P_Interact.P_Interact_C"))
      (set `self.Interact prompt` _returnvalue))
    (:`then_1`
      (bind _returnvalue_2 (`|CreateWidget` "/Game/Blueprints/Crops/WBP_PlantSeed.WBP_PlantSeed_C"))
      (set `self.SeedUI` _returnvalue_2))))

(event `/Game/Blueprints/Interact_BPI.Interact`
  (params (`Player Character` :type "/Game/ThirdPerson/Blueprints/BP_Player_Character Object Reference"))
  (bind _returnvalue (`SceneComponent.K2_GetComponentLocation` (`self.StaticMeshComponent`)))
  ;[1 1 1] Interaction - Fertilize Soil/Open UI
  (if (not (`self.IsFertilized`))
    (bind _result (`self.FertilizerCheck` `Player Character`))
    (if _result
      (`GameplayStatics.SpawnSoundAtLocation` "/Game/SFX/Hoe.Hoe" _returnvalue (struct) 1.0 1.0 0.0 null null)
      (`PrimitiveComponent.SetMaterial` (`self.StaticMeshComponent`) 0 "/Game/Materials/M_Dirt.M_Dirt")
      (set `self.IsFertilized` true)
      (set `/Game/ThirdPerson/Blueprints/BP_Player_Character.DoesTakeEnergy` false `Player Character`)
      (bind _output_get (set `self.FertilizeObjectiveQuantity` (+ (`self.FertilizeObjectiveQuantity`) 1)))
      (`/Game/ThirdPerson/Blueprints/BP_Player_Character.OnObjectiveIDCalled` `Player Character` "fertilizesoil" _output_get)
      (`|SpawnActorFromClass` "/Game/Blueprints/QuestSystem/LocationMarker_BP.LocationMarker_BP_C" (`KismetMathLibrary.MakeTransform` _returnvalue (struct) (5.0 5.0 1.0)) "Undefined" "MultiplyWithRoot" null (`self.LocationName`) (`self.ObjectiveID`) null))
    (elif (`self.UIOpen`)
      ;[1 1 1] Interact Action and Text
      (`Widget.RemoveFromParent` (`self.SeedUI`) :!label _label)
      (else
        (`UserWidget.AddToViewport` (`self.SeedUI`) 0)))))

(event `self.Box.OnComponentBeginOverlap`
  (params (OverlappedComponent :type "PrimitiveComponent Object Reference") (OtherActor :type "Actor Object Reference") (OtherComp :type "PrimitiveComponent Object Reference") (OtherBodyIndex :type Integer) (bFromSweep :type Boolean) (SweepResult :type "HitResult Structure (by ref)"))
  ;[1 1 1] Interact Action and Text
  (if (== OtherActor (`GameplayStatics.GetPlayerCharacter` 0))
    (`UserWidget.AddToViewport` (`self.Interact prompt`) 0)
    (set `/Game/ThirdPerson/Blueprints/BP_Player_Character.NextToInteractable` true (`/Game/Blueprints/Common_BPFL.GetMyPlayerCharacter`))))

(event `self.Box.OnComponentEndOverlap`
  (params (OverlappedComponent :type "PrimitiveComponent Object Reference") (OtherActor :type "Actor Object Reference") (OtherComp :type "PrimitiveComponent Object Reference") (OtherBodyIndex :type Integer))
  ;[1 1 1] Interact Action and Text
  (if (== (`GameplayStatics.GetPlayerCharacter` 0) OtherActor)
    (`Widget.RemoveFromParent` (`self.Interact prompt`))
    (if (`self.UIOpen`)
      (goto _label))))

(fn `FertilizerCheck`
  (params (InputPin :type "/Game/ThirdPerson/Blueprints/BP_Player_Character Object Reference"))
  (returns (Result :type Boolean))
  (bind (_item _success) (`/Game/ThirdPerson/Blueprints/BP_Player_Character.GetItem` InputPin "NewEnumerator1"))
  (if _success
    (`/Game/Blueprints/Interact_BPI.TakePlayerEnergy` InputPin true)
    (bind _result (`/Game/ThirdPerson/Blueprints/BP_Player_Character.RemoveFromInventory` (`local.InputPin`) _item 1))
    (return _result)
    (else
      (bind _output_get (set `self.IsFertilized` false))
      (return _output_get))))

(fn `InteractWith`
  (returns (ObjectiveID :type String))
  (return ""))

(fn `SeedCheck`
  (params (Player :type "/Game/ThirdPerson/Blueprints/BP_Player_Character Object Reference"))
  (returns (Output_Get :type Boolean))
  (bind (_item _success) (`/Game/ThirdPerson/Blueprints/BP_Player_Character.GetItem` Player "NewEnumerator0"))
  (if _success
    (bind _result (`/Game/ThirdPerson/Blueprints/BP_Player_Character.RemoveFromInventory` Player _item 1))
    (return _result)
    (else
      (bind _output_get (set `/Game/ThirdPerson/Blueprints/BP_Player_Character.DoesTakeEnergy` false Player))
      (return _output_get))))

(fn `TakePlayerEnergy`
  (params (isHarvestable :type Boolean))
  (returns (HasEnergy :type Boolean))
  (return false))

(fn `UserConstructionScript`)