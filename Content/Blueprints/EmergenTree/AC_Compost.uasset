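; Composter component that takes kiwis from the player's inventory and hands back compost.
; ReceiveKiwis consumes the kiwis when the bin is empty, plays a sound and reports the "loadbin" objective.
; ProduceCompost checks four composter widgets in EMTUI and passes the compost amount to the UI, but its timer setup here is disconnected.
; TryGiveCompost adds compost to the inventory; status and interaction functions are stubs.
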(fn `CheckComposterStatus`
  (`|ExecutionSequence`
    (:`then_0`
      (`|ExecutionSequence`
        (:`then_0`
          (if (`self.FertilizerReady`)
            _))
        (:`then_1`
          (bind _emt_ui (`self.EMT UI`)
            (:`then`)
            (:`else`)))))))

(fn `InteractWith`
  (returns (ObjectiveID :type String))
  (return ""))

(fn `ProduceCompost`
  (`|ExecutionSequence`
    (:`then_0`
      (if (`/Game/Blueprints/EmergenTree/Emergentree_UI/WB_Composter.IsLoaded` (`/Game/Blueprints/EmergenTree/Emergentree_UI/WB_EMT_UI.WB_Composter` (`self.EMT UI`)))
        (set `self.IsLoaded` false)
        (bind _emt_ui (`self.EMT UI`)
          (:`then`
            (`/Game/Blueprints/EmergenTree/Emergentree_UI/WB_EMT_UI.GetIsCompostReady` _emt_ui (`self.CompostAmount`)))
          (:`else`))))
    (:`then_1`
      (if (`/Game/Blueprints/EmergenTree/Emergentree_UI/WB_Composter.IsLoaded` (`/Game/Blueprints/EmergenTree/Emergentree_UI/WB_EMT_UI.WB_Composter_204` (`self.EMT UI`)))
        (set `self.IsLoaded` false)
        (bind _emt_ui_2 (`self.EMT UI`)
          (:`then`
            (`/Game/Blueprints/EmergenTree/Emergentree_UI/WB_EMT_UI.GetIsCompostReady` _emt_ui_2 (`self.CompostAmount`)))
          (:`else`))))
    (:`then_2`
      (if (`/Game/Blueprints/EmergenTree/Emergentree_UI/WB_Composter.IsLoaded` (`/Game/Blueprints/EmergenTree/Emergentree_UI/WB_EMT_UI.WB_Composter_322` (`self.EMT UI`)))
        (set `self.IsLoaded` false)
        (bind _emt_ui_3 (`self.EMT UI`)
          (:`then`
            (`/Game/Blueprints/EmergenTree/Emergentree_UI/WB_EMT_UI.GetIsCompostReady` _emt_ui_3 (`self.CompostAmount`)))
          (:`else`))))
    (:`then_3`
      (if (`/Game/Blueprints/EmergenTree/Emergentree_UI/WB_Composter.IsLoaded` (`/Game/Blueprints/EmergenTree/Emergentree_UI/WB_EMT_UI.WB_Composter_92` (`self.EMT UI`)))
        (set `self.IsLoaded` false)
        (bind _emt_ui_4 (`self.EMT UI`)
          (:`then`
            (`/Game/Blueprints/EmergenTree/Emergentree_UI/WB_EMT_UI.GetIsCompostReady` _emt_ui_4 (`self.CompostAmount`)))
          (:`else`))))))

(fn `ReceiveKiwis`
  (params (PlayerCharacter :type "/Game/ThirdPerson/Blueprints/BP_Player_Character Object Reference") (ComposterLoaded :type Boolean))
  (returns (IsLoaded :type Boolean))
  (bind _newinventory (`/Game/ThirdPerson/Blueprints/BP_Player_Character.NewInventory` PlayerCharacter))
  (if (and (<= (`self.InventoryCompost`) 0) (not ComposterLoaded))
    (bind _hasitem (`/Game/Blueprints/Inventory/Inventory.HasItemInInventory` _newinventory "NewEnumerator0"))
    (if _hasitem
      (`/Game/Blueprints/Inventory/Inventory.Consume From Inventory` _newinventory "NewEnumerator0" (`self.KiwiAmount`))
      (`GameplayStatics.SpawnSoundAtLocation` "/Game/SFX/Apple_Falls.Apple_Falls" (`Actor.K2_GetActorLocation` (`self.GetOwner`)) (struct) 1.0 1.0 0.0 null null)
      (set `self.InventoryKiwis` (`self.KiwiAmount`))
      (bind _output_get (set `self.IsLoaded` true))
      (`/Game/ThirdPerson/Blueprints/BP_Player_Character.OnObjectiveIDCalled` PlayerCharacter "loadbin" 1)
      (return _output_get)
      (else
        (bind _output_get_2 (set `self.IsLoaded` false))
        (return _output_get_2)))))

(fn `TakePlayerEnergy`
  (params (isHarvestable :type Boolean))
  (returns (HasEnergy :type Boolean))
  (return false))

(fn `Try Give Compost`
  (params (PlayerCharacter :type "/Game/ThirdPerson/Blueprints/BP_Player_Character Object Reference"))
  (`/Game/Blueprints/Inventory/Inventory.AddToInventory` (`/Game/ThirdPerson/Blueprints/BP_Player_Character.NewInventory` PlayerCharacter) "NewEnumerator10" (`self.CompostAmount`))
  (set `self.FertilizerReady` false)
  (return))