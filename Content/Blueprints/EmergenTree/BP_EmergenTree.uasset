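; Interactable Emergen Tree that grows five kiwi types and hosts a composter, both upgradable through five levels with inventory compost.
; Overlapping shows a prompt and links the composter component to the player's tree UI, which interacting toggles.
; Data tables set yields and timings per level, and level-ups call TakePlayerEnergy.
; A half-second timer polls the HUD day, updates UI kiwi amounts when ready, and reschedules growth after harvest.
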(event `self.ReceiveBeginPlay`
  (bind _playercharacter (`/Game/Blueprints/Common_BPFL.GetMyPlayerCharacter`))
  ;[1 1 1] Upgrade Tree On Plant to Level 1
  (`|ExecutionSequence`
    (:`then_0`
      (`self.Production Level Up` _playercharacter)
      (bind _returnvalue (`KismetSystemLibrary.K2_SetTimer` null "CheckGrowthTime" 0.5 true))
      (set `self.CheckGrowthTimer` _returnvalue)
      (`self.ComposterLevelUp` _playercharacter))
    (:`then_1`
      (bind _returnvalue_2 (`|CreateWidget` "/Game/P_Interact.P_Interact_C"))
      (set `self.Interact prompt` _returnvalue_2))))

(event `/Game/Blueprints/Interact_BPI.Interact`
  (params (`Player Character` :type "/Game/ThirdPerson/Blueprints/BP_Player_Character Object Reference"))
  ;[1 1 1] Open UI
  (set `self.PlayerCharacter` `Player Character`)
  (if (`self.UIOpen`)
    ;[1 1 1] Interact Action and Text
    (`Widget.SetVisibility` (`/Game/ThirdPerson/Blueprints/BP_Player_Character.WB EMT UI` (`self.PlayerCharacter`)) "Hidden" :!label _label)
    (set `self.UIOpen` false)
    (else
      (`Widget.SetVisibility` (`self.EmergentreeUI`) "Visible")
      (set `self.UIOpen` true))))

(event `self.Sphere.OnComponentBeginOverlap`
  (params (OverlappedComponent :type "PrimitiveComponent Object Reference") (OtherActor :type "Actor Object Reference") (OtherComp :type "PrimitiveComponent Object Reference") (OtherBodyIndex :type Integer) (bFromSweep :type Boolean) (SweepResult :type "HitResult Structure (by ref)"))
  (bind _playercharacter (`/Game/Blueprints/Common_BPFL.GetMyPlayerCharacter`))
  (bind _ac_compost (`self.AC_Compost`))
  (bind _wb_emt_ui (`/Game/ThirdPerson/Blueprints/BP_Player_Character.WB EMT UI` _playercharacter))
  ;[1 1 1] Interact Action and Text
  (if (== OtherActor (`GameplayStatics.GetPlayerCharacter` 0))
    (`UserWidget.AddToViewport` (`self.Interact prompt`) 0)
    (set `/Game/ThirdPerson/Blueprints/BP_Player_Character.NextToInteractable` true _playercharacter)
    (set `self.EmergentreeUI` _wb_emt_ui)
    (`/Engine/EditorBlueprintResources/StandardMacros.DoOnce` false
      (:`Completed`
        (set `/Game/Blueprints/EmergenTree/Emergentree_UI/WB_EMT_UI.AC_Compost` _ac_compost _wb_emt_ui)
        (set `/Game/Blueprints/EmergenTree/AC_Compost.EMT UI` _wb_emt_ui _ac_compost)
        (`/Game/Blueprints/EmergenTree/Emergentree_UI/WB_EMT_UI.InitializeComposterNodes` _wb_emt_ui)))))

(event `self.Sphere.OnComponentEndOverlap`
  (params (OverlappedComponent :type "PrimitiveComponent Object Reference") (OtherActor :type "Actor Object Reference") (OtherComp :type "PrimitiveComponent Object Reference") (OtherBodyIndex :type Integer))
  ;[1 1 1] Interact Action and Text
  (if (== (`GameplayStatics.GetPlayerCharacter` 0) OtherActor)
    (`Widget.RemoveFromParent` (`self.Interact prompt`))
    (if (`self.UIOpen`)
      (goto _label))))

(fn `CheckGrowthTime`
  (locals (Day :type Integer))
  (bind _foundwidgets (`WidgetBlueprintLibrary.GetAllWidgetsOfClass` "/Game/ThirdPerson/HUD/WBP_HUD.WBP_HUD_C"))
  (bind _day (`/Game/ThirdPerson/HUD/WBP_HUD.GetDayInt` _foundwidgets))
  (set `local.Day` _day)
  (`|ExecutionSequence`
    (:`then_0`
      ;[1 1 1] Small Kiwi Check
      (`|ExecutionSequence`
        (:`then_0`
          (if (== (`local.Day`) (`self.SmallKiwiGrowthDay`))
            (`self.SpawnSmallKiwis`)
            (set `self.SmallKiwiGrowthDay` 0)
            (bind _wb_fruit_node_1 (`/Game/Blueprints/EmergenTree/Emergentree_UI/WB_EMT_UI.WB_Fruit_Node_1` (stale _emergentreeui)))
            (bind _isharvestable (`/Game/Blueprints/EmergenTree/Emergentree_UI/WB_Fruit_Node.CheckIfKiwiReady` _wb_fruit_node_1))
            (if _isharvestable
              (bind _emergentreeui (`self.EmergentreeUI`)
                (:`then`
                  (set `/Game/Blueprints/EmergenTree/Emergentree_UI/WB_Fruit_Node.Texture` "/Game/Blueprints/EmergenTree/Emergentree_UI/UI_Assets/fruit-node-full.fruit-node-full" _wb_fruit_node_1)
                  (set `TextBlock.Text` "HARVEST" (`/Game/Blueprints/EmergenTree/Emergentree_UI/WB_Fruit_Node.TextBlock_0` _wb_fruit_node_1)))
                (:`else`)))))
        (:`then_1`
          (bind _emergentreeui_2 (`self.EmergentreeUI`)
            (:`then`
              (bind _harvested_ (`/Game/Blueprints/EmergenTree/Emergentree_UI/WB_EMT_UI.GetIfKiwiHarvested` _emergentreeui_2 "Small"))
              (if _harvested_
                (bind _newgrowthday (`self.Set New Growth Day`))
                (set `self.SmallKiwiGrowthDay` _newgrowthday)
                (`/Game/Blueprints/EmergenTree/Emergentree_UI/WB_EMT_UI.SetKiwiHarvested` _emergentreeui_2 "Small" false)
                (bind _emergentreeui_3 (`self.EmergentreeUI`)
                  (:`then`
                    (bind _wb_fruit_node_1_2 (`/Game/Blueprints/EmergenTree/Emergentree_UI/WB_EMT_UI.WB_Fruit_Node_1` _emergentreeui_3))
                    (set `/Game/Blueprints/EmergenTree/Emergentree_UI/WB_Fruit_Node.Texture` "/Game/Blueprints/EmergenTree/Emergentree_UI/UI_Assets/fruit-node-sapling.fruit-node-sapling" _wb_fruit_node_1_2)
                    (set `TextBlock.Text` "Not Ready" (`/Game/Blueprints/EmergenTree/Emergentree_UI/WB_Fruit_Node.TextBlock_0` _wb_fruit_node_1_2)))
                  (:`else`))))
            (:`else`)))))
    (:`then_1`
      ;[1 1 1] Big Kiwi Check
      (`|ExecutionSequence`
        (:`then_0`
          (if (== (`local.Day`) (`self.BigKiwiGrowthDay`))
            (`self.SpawnBigKiwis`)
            (set `self.BigKiwiGrowthDay` 0)
            (bind _wb_fruit_node_2 (`/Game/Blueprints/EmergenTree/Emergentree_UI/WB_EMT_UI.WB_Fruit_Node_2` (stale _emergentreeui_4)))
            (bind _isharvestable_2 (`/Game/Blueprints/EmergenTree/Emergentree_UI/WB_Fruit_Node.CheckIfKiwiReady` _wb_fruit_node_2))
            (if _isharvestable_2
              (bind _emergentreeui_4 (`self.EmergentreeUI`)
                (:`then`
                  (set `/Game/Blueprints/EmergenTree/Emergentree_UI/WB_Fruit_Node.Texture` "/Game/Blueprints/EmergenTree/Emergentree_UI/UI_Assets/fruit-node-full.fruit-node-full" _wb_fruit_node_2)
                  (set `TextBlock.Text` "HARVEST" (`/Game/Blueprints/EmergenTree/Emergentree_UI/WB_Fruit_Node.TextBlock_0` _wb_fruit_node_2)))
                (:`else`)))))
        (:`then_1`
          (bind _emergentreeui_5 (`self.EmergentreeUI`)
            (:`then`
              (bind _harvested__2 (`/Game/Blueprints/EmergenTree/Emergentree_UI/WB_EMT_UI.GetIfKiwiHarvested` _emergentreeui_5 "Big"))
              (if _harvested__2
                (bind _newgrowthday_2 (`self.Set New Growth Day`))
                (set `self.BigKiwiGrowthDay` _newgrowthday_2)
                (`/Game/Blueprints/EmergenTree/Emergentree_UI/WB_EMT_UI.SetKiwiHarvested` _emergentreeui_5 "Big" false)
                (bind _emergentreeui_6 (`self.EmergentreeUI`)
                  (:`then`
                    (bind _wb_fruit_node_2_2 (`/Game/Blueprints/EmergenTree/Emergentree_UI/WB_EMT_UI.WB_Fruit_Node_2` _emergentreeui_6))
                    (set `/Game/Blueprints/EmergenTree/Emergentree_UI/WB_Fruit_Node.Texture` "/Game/Blueprints/EmergenTree/Emergentree_UI/UI_Assets/fruit-node-sapling.fruit-node-sapling" _wb_fruit_node_2_2)
                    (set `TextBlock.Text` "Not Ready" (`/Game/Blueprints/EmergenTree/Emergentree_UI/WB_Fruit_Node.TextBlock_0` _wb_fruit_node_2_2)))
                  (:`else`))))
            (:`else`)))))
    (:`then_2`
      ;[1 1 1] Metal Kiwi Check
      (`|ExecutionSequence`
        (:`then_0`
          (if (== (`local.Day`) (`self.MetalKiwiGrowthDay`))
            (`self.SpawnMetalKiwis`)
            (set `self.MetalKiwiGrowthDay` 0)
            (bind _wb_fruit_node_3 (`/Game/Blueprints/EmergenTree/Emergentree_UI/WB_EMT_UI.WB_Fruit_Node_3` (stale _emergentreeui_7)))
            (bind _isharvestable_3 (`/Game/Blueprints/EmergenTree/Emergentree_UI/WB_Fruit_Node.CheckIfKiwiReady` _wb_fruit_node_3))
            (if _isharvestable_3
              (bind _emergentreeui_7 (`self.EmergentreeUI`)
                (:`then`
                  (set `/Game/Blueprints/EmergenTree/Emergentree_UI/WB_Fruit_Node.Texture` "/Game/Blueprints/EmergenTree/Emergentree_UI/UI_Assets/fruit-node-full.fruit-node-full" _wb_fruit_node_3)
                  (set `TextBlock.Text` "HARVEST" (`/Game/Blueprints/EmergenTree/Emergentree_UI/WB_Fruit_Node.TextBlock_0` _wb_fruit_node_3)))
                (:`else`)))))
        (:`then_1`
          (bind _emergentreeui_8 (`self.EmergentreeUI`)
            (:`then`
              (bind _harvested__3 (`/Game/Blueprints/EmergenTree/Emergentree_UI/WB_EMT_UI.GetIfKiwiHarvested` _emergentreeui_8 "Metal"))
              (if _harvested__3
                (bind _newgrowthday_3 (`self.Set New Growth Day`))
                (set `self.MetalKiwiGrowthDay` _newgrowthday_3)
                (`/Game/Blueprints/EmergenTree/Emergentree_UI/WB_EMT_UI.SetKiwiHarvested` _emergentreeui_8 "Metal" false)
                (bind _emergentreeui_9 (`self.EmergentreeUI`)
                  (:`then`
                    (bind _wb_fruit_node_3_2 (`/Game/Blueprints/EmergenTree/Emergentree_UI/WB_EMT_UI.WB_Fruit_Node_3` _emergentreeui_9))
                    (set `/Game/Blueprints/EmergenTree/Emergentree_UI/WB_Fruit_Node.Texture` "/Game/Blueprints/EmergenTree/Emergentree_UI/UI_Assets/fruit-node-sapling.fruit-node-sapling" _wb_fruit_node_3_2)
                    (set `TextBlock.Text` "Not Ready" (`/Game/Blueprints/EmergenTree/Emergentree_UI/WB_Fruit_Node.TextBlock_0` _wb_fruit_node_3_2)))
                  (:`else`))))
            (:`else`)))))
    (:`then_3`
      ;[1 1 1] Icey Kiwi Check
      (`|ExecutionSequence`
        (:`then_0`
          (if (== (`local.Day`) (`self.IceyKiwiGrowthDay`))
            (`self.SpawnIceyKiwis`)
            (set `self.IceyKiwiGrowthDay` 0)
            (bind _wb_fruit_node_4 (`/Game/Blueprints/EmergenTree/Emergentree_UI/WB_EMT_UI.WB_Fruit_Node_4` (stale _emergentreeui_10)))
            (bind _isharvestable_4 (`/Game/Blueprints/EmergenTree/Emergentree_UI/WB_Fruit_Node.CheckIfKiwiReady` _wb_fruit_node_4))
            (if _isharvestable_4
              (bind _emergentreeui_10 (`self.EmergentreeUI`)
                (:`then`
                  (set `/Game/Blueprints/EmergenTree/Emergentree_UI/WB_Fruit_Node.Texture` "/Game/Blueprints/EmergenTree/Emergentree_UI/UI_Assets/fruit-node-full.fruit-node-full" _wb_fruit_node_4)
                  (set `TextBlock.Text` "HARVEST" (`/Game/Blueprints/EmergenTree/Emergentree_UI/WB_Fruit_Node.TextBlock_0` _wb_fruit_node_4)))
                (:`else`)))))
        (:`then_1`
          (bind _emergentreeui_11 (`self.EmergentreeUI`)
            (:`then`
              (bind _harvested__4 (`/Game/Blueprints/EmergenTree/Emergentree_UI/WB_EMT_UI.GetIfKiwiHarvested` _emergentreeui_11 "Icey"))
              (if _harvested__4
                (bind _newgrowthday_4 (`self.Set New Growth Day`))
                (set `self.IceyKiwiGrowthDay` _newgrowthday_4)
                (`/Game/Blueprints/EmergenTree/Emergentree_UI/WB_EMT_UI.SetKiwiHarvested` _emergentreeui_11 "Icey" false)
                (bind _emergentreeui_12 (`self.EmergentreeUI`)
                  (:`then`
                    (bind _wb_fruit_node_4_2 (`/Game/Blueprints/EmergenTree/Emergentree_UI/WB_EMT_UI.WB_Fruit_Node_4` _emergentreeui_12))
                    (set `/Game/Blueprints/EmergenTree/Emergentree_UI/WB_Fruit_Node.Texture` "/Game/Blueprints/EmergenTree/Emergentree_UI/UI_Assets/fruit-node-sapling.fruit-node-sapling" _wb_fruit_node_4_2)
                    (set `TextBlock.Text` "Not Ready" (`/Game/Blueprints/EmergenTree/Emergentree_UI/WB_Fruit_Node.TextBlock_0` _wb_fruit_node_4_2)))
                  (:`else`))))
            (:`else`)))))
    (:`then_4`
      ;[1 1 1] Heated Kiwi Check
      (`|ExecutionSequence`
        (:`then_0`
          (if (== (`local.Day`) (`self.HeatedKiwiGrowthDay`))
            (`self.SpawnHeatedKiwis`)
            (set `self.HeatedKiwiGrowthDay` 0)
            (bind _wb_fruit_node_5 (`/Game/Blueprints/EmergenTree/Emergentree_UI/WB_EMT_UI.WB_Fruit_Node_5` (stale _emergentreeui_13)))
            (bind _isharvestable_5 (`/Game/Blueprints/EmergenTree/Emergentree_UI/WB_Fruit_Node.CheckIfKiwiReady` _wb_fruit_node_5))
            (if _isharvestable_5
              (bind _emergentreeui_13 (`self.EmergentreeUI`)
                (:`then`
                  (set `/Game/Blueprints/EmergenTree/Emergentree_UI/WB_Fruit_Node.Texture` "/Game/Blueprints/EmergenTree/Emergentree_UI/UI_Assets/fruit-node-full.fruit-node-full" _wb_fruit_node_5)
                  (set `TextBlock.Text` "HARVEST" (`/Game/Blueprints/EmergenTree/Emergentree_UI/WB_Fruit_Node.TextBlock_0` _wb_fruit_node_5)))
                (:`else`)))))
        (:`then_1`
          (bind _emergentreeui_14 (`self.EmergentreeUI`)
            (:`then`
              (bind _harvested__5 (`/Game/Blueprints/EmergenTree/Emergentree_UI/WB_EMT_UI.GetIfKiwiHarvested` _emergentreeui_14 "Heated"))
              (if _harvested__5
                (bind _newgrowthday_5 (`self.Set New Growth Day`))
                (set `self.HeatedKiwiGrowthDay` _newgrowthday_5)
                (`/Game/Blueprints/EmergenTree/Emergentree_UI/WB_EMT_UI.SetKiwiHarvested` _emergentreeui_14 "Heated" false)
                (bind _emergentreeui_15 (`self.EmergentreeUI`)
                  (:`then`
                    (bind _wb_fruit_node_5_2 (`/Game/Blueprints/EmergenTree/Emergentree_UI/WB_EMT_UI.WB_Fruit_Node_5` _emergentreeui_15))
                    (set `/Game/Blueprints/EmergenTree/Emergentree_UI/WB_Fruit_Node.Texture` "/Game/Blueprints/EmergenTree/Emergentree_UI/UI_Assets/fruit-node-sapling.fruit-node-sapling" _wb_fruit_node_5_2)
                    (set `TextBlock.Text` "Not Ready" (`/Game/Blueprints/EmergenTree/Emergentree_UI/WB_Fruit_Node.TextBlock_0` _wb_fruit_node_5_2)))
                  (:`else`))))
            (:`else`)))))))

(fn `ComposterLevelUp`
  (params (`Player Character` :type "/Game/ThirdPerson/Blueprints/BP_Player_Character Object Reference"))
  (switch `name` (`self.CurrentTreeCompostLvl`)
    (:`0`
      (set `self.CurrentTreeCompostLvl` "Level1"))
    (:`Level1`
      (set `self.CurrentTreeCompostLvl` "Level2"))
    (:`Level2`
      (set `self.CurrentTreeCompostLvl` "Level3"))
    (:`Level3`
      (set `self.CurrentTreeCompostLvl` "Level4"))
    (:`Level4`
      (set `self.CurrentTreeCompostLvl` "Level5")
      (set `self.MaxComposterLvlReached` true)))
  (`/Game/Blueprints/Interact_BPI.TakePlayerEnergy` `Player Character` true)
  (`self.FetchCompostYieldLvlData`)
  (`KismetSystemLibrary.PrintString` (`KismetStringLibrary.Concat_StrStr` "Current Level: " (`KismetStringLibrary.Conv_NameToString` (`self.CurrentTreeCompostLvl`)))))

(fn `Fetch Production Yield Lvl Data`
  (bind _returnvalue (`|GetDataTableRow` "/Game/Blueprints/EmergenTree/EmergenTreeLevels/KiwiYieldLevels.KiwiYieldLevels" (`self.CurrentTreeProductionLvl`))
    (:`then`
      (bind (_daystoyield _compostamtneededfornxtlvl _smallkiwiamount _bigkiwiamount _metalkiwiamount _iceykiwiamount _heatedkiwiamount) (break `/Game/Blueprints/EmergenTree/EmergenTreeLevels/KiwiYieldData` _returnvalue))
      (set `self.DaysToYield` _daystoyield)
      (set `self.CompostToProductionLvlUp` _compostamtneededfornxtlvl)
      (set `self.MaxSmallKiwiAmount` _smallkiwiamount)
      (set `self.MaxBigKiwiAmount` _bigkiwiamount)
      (set `self.MaxMetalKiwiAmount` _metalkiwiamount)
      (set `self.MaxIceyKiwiAmount` _iceykiwiamount)
      (set `self.MaxHeatedKiwiAmount` _heatedkiwiamount))))

(fn `FetchCompostYieldLvlData`
  (bind _ac_compost (`self.AC_Compost`))
  (bind _returnvalue (`|GetDataTableRow` "/Game/Blueprints/EmergenTree/EmergenTreeLevels/CompostYieldLevels.CompostYieldLevels" (`self.CurrentTreeCompostLvl`))
    (:`then`
      (bind (_timetoyield _compostamtneededfornxtlvl _kiwiamount _compostamount) (break `/Game/Blueprints/EmergenTree/EmergenTreeLevels/CompostYieldData` _returnvalue))
      (bind _output_get (set `self.TimeToYield` _timetoyield))
      (set `/Game/Blueprints/EmergenTree/AC_Compost.ComposterTime` _output_get _ac_compost)
      (set `self.CompostToComposterLvlUp` _compostamtneededfornxtlvl)
      (bind _output_get_2 (set `self.KiwiAmount` _kiwiamount))
      (set `/Game/Blueprints/EmergenTree/AC_Compost.KiwiAmount` _output_get_2 _ac_compost)
      (bind _output_get_3 (set `self.CompostAmount` _compostamount))
      (set `/Game/Blueprints/EmergenTree/AC_Compost.CompostAmount` _output_get_3 _ac_compost))))

(fn `InteractWith`
  (returns (ObjectiveID :type String))
  (return ""))

(fn `Production Level Up`
  (params (`Player Character` :type "/Game/ThirdPerson/Blueprints/BP_Player_Character Object Reference"))
  (switch `name` (`self.CurrentTreeProductionLvl`)
    (:`0`
      (set `self.CurrentTreeProductionLvl` "Lvl1")
      (`/Game/Blueprints/Interact_BPI.TakePlayerEnergy` `Player Character` true :!label _label)
      (`self.Fetch Production Yield Lvl Data`)
      (bind _newgrowthday (`self.Set New Growth Day`))
      (bind _output_get (set `self.SmallKiwiGrowthDay` _newgrowthday))
      (bind _output_get_2 (set `self.BigKiwiGrowthDay` _output_get))
      (bind _output_get_3 (set `self.MetalKiwiGrowthDay` _output_get_2))
      (bind _output_get_4 (set `self.IceyKiwiGrowthDay` _output_get_3))
      (set `self.HeatedKiwiGrowthDay` _output_get_4))
    (:`Lvl1`
      (set `self.CurrentTreeProductionLvl` "Lvl2")
      (goto _label))
    (:`Lvl2`
      (set `self.CurrentTreeProductionLvl` "Lvl3")
      (goto _label))
    (:`Lvl3`
      (set `self.CurrentTreeProductionLvl` "Lvl4")
      (goto _label))
    (:`Lvl4`
      (set `self.CurrentTreeProductionLvl` "Lvl5")
      (set `self.MaxProductionLevelReached` true)
      (`/Game/Blueprints/Interact_BPI.TakePlayerEnergy` `Player Character` true)
      (`self.Fetch Production Yield Lvl Data`)
      (`KismetSystemLibrary.PrintString` "Max Lvl. Reached"))))

(fn `Set New Growth Day`
  (returns (NewGrowthDay :type Integer))
  (bind _foundwidgets (`WidgetBlueprintLibrary.GetAllWidgetsOfClass` "/Game/ThirdPerson/HUD/WBP_HUD.WBP_HUD_C"))
  (bind _day (`/Game/ThirdPerson/HUD/WBP_HUD.GetDayInt` _foundwidgets))
  (return (+ _day (`self.DaysToYield`))))

(fn `SpawnBigKiwis`
  (`/Game/Blueprints/EmergenTree/Emergentree_UI/WB_EMT_UI.UpdateBigKiwiAmount` (`self.EmergentreeUI`) (`self.MaxBigKiwiAmount`)))

(fn `SpawnHeatedKiwis`
  (`/Game/Blueprints/EmergenTree/Emergentree_UI/WB_EMT_UI.UpdateHeatedKiwiAmount` (`self.EmergentreeUI`) (`self.MaxHeatedKiwiAmount`)))

(fn `SpawnIceyKiwis`
  (`/Game/Blueprints/EmergenTree/Emergentree_UI/WB_EMT_UI.UpdateIceyKiwiAmount` (`self.EmergentreeUI`) (`self.MaxIceyKiwiAmount`)))

(fn `SpawnMetalKiwis`
  (`/Game/Blueprints/EmergenTree/Emergentree_UI/WB_EMT_UI.UpdateMetalKiwiAmount` (`self.EmergentreeUI`) (`self.MaxMetalKiwiAmount`)))

(fn `SpawnSmallKiwis`
  (bind _emergentreeui (`self.EmergentreeUI`)
    (:`then`
      (`/Game/Blueprints/EmergenTree/Emergentree_UI/WB_EMT_UI.UpdateSmallKiwiAmount` _emergentreeui (`self.MaxSmallKiwiAmount`)))
    (:`else`)))

(fn `TakePlayerEnergy`
  (params (isHarvestable :type Boolean))
  (returns (HasEnergy :type Boolean))
  (return false))

(fn `Upgrade Production With Compost`
  (bind _playercharacter (`self.PlayerCharacter`))
  (bind _composttoproductionlvlup (`self.CompostToProductionLvlUp`))
  (if (not (`self.MaxProductionLevelReached`))
    (bind _hasitem (`/Game/Blueprints/Inventory/Inventory.Check Item Amount in Inventory` (`/Game/ThirdPerson/Blueprints/BP_Player_Character.NewInventory` _playercharacter) "NewEnumerator10" _composttoproductionlvlup))
    (if _hasitem
      (`/Game/Blueprints/Inventory/Inventory.Consume From Inventory` (`/Game/ThirdPerson/Blueprints/BP_Player_Character.NewInventory` _playercharacter) "NewEnumerator10" _composttoproductionlvlup)
      (`self.Production Level Up` _playercharacter)
      (`/Game/Blueprints/EmergenTree/Emergentree_UI/WB_EMT_UI.Unlock Next Tree Production Lvl` (`self.EmergentreeUI`) (`self.CurrentTreeProductionLvl`))
      (`KismetSystemLibrary.K2_ClearAndInvalidateTimerHandle` (`self.CheckGrowthTimer`))
      (`KismetSystemLibrary.K2_SetTimer` null "CheckGrowthTime" 0.5 true)
      (else
        (`KismetSystemLibrary.PrintString` "Not Enough Compost")))))

(fn `UpgradeComposterWithCompost`
  (bind _composttocomposterlvlup (`self.CompostToComposterLvlUp`))
  (bind _newinventory (`/Game/ThirdPerson/Blueprints/BP_Player_Character.NewInventory` (`self.PlayerCharacter`)))
  (if (not (`self.MaxComposterLvlReached`))
    (bind _hasitem (`/Game/Blueprints/Inventory/Inventory.Check Item Amount in Inventory` _newinventory "NewEnumerator10" _composttocomposterlvlup))
    (if _hasitem
      (`/Game/Blueprints/Inventory/Inventory.Consume From Inventory` _newinventory "NewEnumerator10" _composttocomposterlvlup)
      (`self.ComposterLevelUp` (`self.PlayerCharacter`))
      (`/Game/Blueprints/EmergenTree/Emergentree_UI/WB_EMT_UI.UnlockNextComposterLvl` (`self.EmergentreeUI`) (`self.CurrentTreeCompostLvl`))
      (else
        (`KismetSystemLibrary.PrintString` "Not Enough Compost")))))

(fn `UserConstructionScript`)