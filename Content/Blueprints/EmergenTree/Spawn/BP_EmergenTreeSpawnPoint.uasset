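; Plantable plot where the player spawns an EmergenTree, showing an interact prompt while the player overlaps its sphere.
; Interact spawns BP_EmergenTree at the plot's transform, disables further planting and adds several item types to the player's inventory, repeated per KiwisOnSpawn.
; Interact's planting condition is hard-coded true; the kit inventory check lives only in a separate PlayerInteractedWithSpawnPoint event.
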(event `self.ReceiveActorBeginOverlap`
  (params (OtherActor :type "Actor Object Reference")))

(event `Event PlayerInteractedWithSpawnPoint`
  (bind _hasitem (`/Game/Blueprints/Inventory/Inventory.HasItemInInventory` (`/Game/ThirdPerson/Blueprints/BP_Player_Character.NewInventory` (`self.PlayerCharacter`)) "NewEnumerator11"))
  (if _hasitem
    (`self.GenerateEmergenTree`)
    (`self.DisablePlot`)
    (else
      (`KismetSystemLibrary.PrintString` "Player has no emergentree kit"))))

(event `/Game/Blueprints/Interact_BPI.Interact`
  (params (`Player Character` :type "/Game/ThirdPerson/Blueprints/BP_Player_Character Object Reference"))
  (bind _playercharacter (`self.PlayerCharacter`))
  (bind _newinventory (`/Game/ThirdPerson/Blueprints/BP_Player_Character.NewInventory` _playercharacter))
  (set `self.PlayerCharacter` `Player Character`)
  (if (`self.isInteractable`)
    (if true
      (`self.GenerateEmergenTree`)
      (`self.DisablePlot`)
      (set `/Game/ThirdPerson/Blueprints/BP_Player_Character.NextToInteractable` false _playercharacter)
      (for _ (range (`self.KiwisOnSpawn`))
        (`/Game/Blueprints/Inventory/Inventory.AddToInventory` _newinventory "NewEnumerator0" 1)
        (`/Game/Blueprints/Inventory/Inventory.AddToInventory` _newinventory "NewEnumerator10" 1)
        (`/Game/Blueprints/Inventory/Inventory.AddToInventory` _newinventory "NewEnumerator5" 1)
        (`/Game/Blueprints/Inventory/Inventory.AddToInventory` _newinventory "NewEnumerator6" 1)
        (`/Game/Blueprints/Inventory/Inventory.AddToInventory` _newinventory "NewEnumerator7" 1)
        (`/Game/Blueprints/Inventory/Inventory.AddToInventory` _newinventory "NewEnumerator8" 1)
        (`/Game/Blueprints/Inventory/Inventory.AddToInventory` _newinventory "NewEnumerator9" 1))
      (else
        (`KismetSystemLibrary.PrintString` "Cannot plant tree")))))

(event `self.ReceiveBeginPlay`
  ;[1 1 1] Interact Action and Text
  (bind _returnvalue (`|CreateWidget` "/Game/P_Interact.P_Interact_C"))
  (bind _output_get (set `self.Interact prompt` _returnvalue))
  (`/Game/P_Interact.SetTextBlock` _output_get "[E] To Plant EmergenTree"))

(event `self.Sphere.OnComponentBeginOverlap`
  (params (OverlappedComponent :type "PrimitiveComponent Object Reference") (OtherActor :type "Actor Object Reference") (OtherComp :type "PrimitiveComponent Object Reference") (OtherBodyIndex :type Integer) (bFromSweep :type Boolean) (SweepResult :type "HitResult Structure (by ref)"))
  ;[1 1 1] Interact Action and Text
  (if (== OtherActor (`GameplayStatics.GetPlayerCharacter` 0))
    (`UserWidget.AddToViewport` (`self.Interact prompt`) 0)
    (if (`self.isInteractable`)
      (bind _asbp_player_character (cast `/Game/ThirdPerson/Blueprints/BP_Player_Character` OtherActor))
      (set `/Game/ThirdPerson/Blueprints/BP_Player_Character.NextToInteractable` true _asbp_player_character))))

(event `self.Sphere.OnComponentEndOverlap`
  (params (OverlappedComponent :type "PrimitiveComponent Object Reference") (OtherActor :type "Actor Object Reference") (OtherComp :type "PrimitiveComponent Object Reference") (OtherBodyIndex :type Integer))
  ;[1 1 1] Interact Action and Text
  (if (== (`GameplayStatics.GetPlayerCharacter` 0) OtherActor)
    (`Widget.RemoveFromParent` (`self.Interact prompt`))))

(fn `DisablePlot`
  (`ActorComponent.K2_DestroyComponent` (`self.Sphere`))
  (set `self.isInteractable` false))

(fn `GenerateEmergenTree`
  (bind (_returnvalue_location _returnvalue_rotation _returnvalue_scale) (`KismetMathLibrary.BreakTransform` (`self.GetTransform`)))
  (`|SpawnActorFromClass` "/Game/Blueprints/EmergenTree/BP_EmergenTree.BP_EmergenTree_C" (`KismetMathLibrary.MakeTransform` _returnvalue_location _returnvalue_rotation _returnvalue_scale) "AlwaysSpawn" "MultiplyWithRoot" self (`self.PlayerCharacter`))
  (`PrimitiveComponent.SetCollisionObjectType` (`self.EmergenTree Plot of Land`) "ECC_GameTraceChannel3"))

(fn `InteractWith`
  (returns (ObjectiveID :type String))
  (return ""))

(fn `TakePlayerEnergy`
  (params (isHarvestable :type Boolean))
  (returns (HasEnergy :type Boolean))
  (return false))

(fn `UserConstructionScript`)