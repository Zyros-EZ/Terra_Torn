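; Inventory Blueprint that tracks how many of each item is held, keyed by item ID in InventoryMap.
; Adding increments the stored count through GetInventoryCount, which treats missing items as zero.
; Consuming checks HasItemInInventory, decrements with a floor of zero, and prints a message when none is available.
; Depleted items stay in the map at zero, so presence checks test for a count above zero.
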(fn `AddToInventory`
  (params (itemId :type String))
  (bind _count (`self.GetInventoryCount` itemId))
  (`BlueprintMapLibrary.Map_Add` (`self.inventoryMap`) itemId (+ _count 1)))

(fn `Consume From Inventory`
  (params (itemId :type String))
  (bind _hasitem (`self.HasItemInInventory` itemId))
  (if _hasitem
    (bind _count (`self.GetInventoryCount` itemId))
    (`BlueprintMapLibrary.Map_Add` (`self.inventoryMap`) itemId (`KismetMathLibrary.Max` (- _count 1)))
    (else
      (`KismetSystemLibrary.PrintString` null "Attempted to consume an item that doesn't exist in the inventory"))))

(fn `GetInventoryCount`
  (params (itemId :type String))
  (returns (count :type Integer))
  (bind (_value _returnvalue) (`BlueprintMapLibrary.Map_Find` (`self.inventoryMap`) itemId))
  (if _returnvalue
    (return _value)
    (else
      (return 0))))

(fn `HasItemInInventory`
  (params (itemId :type String))
  (returns (hasItem :type Boolean))
  (bind (_value _returnvalue) (`BlueprintMapLibrary.Map_Find` (`self.inventoryMap`) itemId))
  (if _returnvalue
    (return (> _value 0))
    (else
      (return false))))