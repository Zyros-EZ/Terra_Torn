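; Item creation factory that instantiates item objects from either an item ID or a crop type.
; CreateByItemId looks up the class in the ItemIdToItem map and constructs a new object from it.
; CreateByCropType translates the crop type to an ID through CropTypeToId, then delegates to CreateByItemId.
; Both functions construct an item only when their map lookup succeeds.
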(fn `Create By Crop Type`
  (params (cropType :type "/Game/Blueprints/Items/Kiwis/CropType Enum" :default "NewEnumerator0"))
  (returns (ReturnValue :type "/Game/Blueprints/Items/Item Object Reference"))
  (bind (_value _returnvalue) (`BlueprintMapLibrary.Map_Find` (`self.cropTypeToId`) cropType))
  (if _returnvalue
    (bind _returnvalue_2 (`self.Create By Item Id` _value))
    (return _returnvalue_2)))

(fn `Create By Item Id`
  (params (id :type String))
  (returns (ReturnValue :type "/Game/Blueprints/Items/Item Object Reference"))
  (bind (_value _returnvalue) (`BlueprintMapLibrary.Map_Find` (`self.itemIdToItem`) id))
  (if _returnvalue
    (bind _returnvalue_2 (`|GenericCreateObject` _value))
    (return _returnvalue_2)))