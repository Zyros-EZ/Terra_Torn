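; ItemFactory creates item objects from either a kiwi type or an item ID.
; Each creation function looks up the class in its own map, KiwiTypeToClass or ItemIdToClass, then constructs an instance with the supplied Owner as outer.
; A failed lookup only prints an invalid-type or invalid-ID message and constructs nothing.
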(fn `CreateItemFromId`
  (params (id :type "/Game/Blueprints/Items/ItemId Enum" :default "NewEnumerator0") (owner :type "Object Object Reference"))
  (returns (item :type "/Game/Blueprints/Items/Item Object Reference"))
  (locals (itemIdToClass :type "Map of /Game/Blueprints/Items/ItemId Enum to /Game/Blueprints/Items/Item Class Reference"))
  (bind (_value _returnvalue) (`BlueprintMapLibrary.Map_Find` (`local.itemIdToClass`) id))
  (if _returnvalue
    (bind _returnvalue_2 (`|GenericCreateObject` owner _value))
    (return _returnvalue_2)
    (else
      (`KismetSystemLibrary.PrintString` null "Invalid item id attempted to be created"))))

(fn `CreateItemFromKiwiType`
  (params (kiwiType :type "/Game/Blueprints/Items/Kiwis/KiwiType Enum" :default "NewEnumerator0") (owner :type "Object Object Reference"))
  (returns (item :type "/Game/Blueprints/Items/Item Object Reference"))
  (locals (kiwiTypeToClass :type "Map of /Game/Blueprints/Items/Kiwis/KiwiType Enum to /Game/Blueprints/Items/Item Class Reference"))
  (bind (_value _returnvalue) (`BlueprintMapLibrary.Map_Find` (`local.kiwiTypeToClass`) kiwiType))
  (if _returnvalue
    (bind _returnvalue_2 (`|GenericCreateObject` owner _value))
    (return _returnvalue_2)
    (else
      (`KismetSystemLibrary.PrintString` null "Invalid kiwi type attempted to be created"))))