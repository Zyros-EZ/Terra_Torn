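; Game instance Blueprint that sets up the game's save data on Init.
; If the save slot exists, it loads it into SaveData as SaveGame_BP, then deletes the slot, so the loaded data remains only in memory.
; Otherwise it creates a fresh SaveGame_BP and adds a starting quest through the player character's quest log component.
; Nothing here writes the save back to disk.
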(event `self.ReceiveInit`
  (bind _slot_name (`self.Slot Name`))
  (bind _returnvalue (`GameplayStatics.DoesSaveGameExist` _slot_name))
  (if _returnvalue
    (bind _returnvalue_2 (`GameplayStatics.LoadGameFromSlot` _slot_name))
    (bind _assave_game_bp (cast `/Game/Blueprints/SaveGame_BP` _returnvalue_2))
    (set `self.SaveData` _assave_game_bp)
    (`GameplayStatics.DeleteGameInSlot` _slot_name)
    (else
      (bind _returnvalue_3 (`GameplayStatics.CreateSaveGameObject` "/Game/Blueprints/SaveGame_BP.SaveGame_BP_C"))
      (set `self.SaveData` _returnvalue_3)
      (`/Game/Blueprints/QuestSystem/QuestLogComponent_BP.AddNewQuest` (`/Game/ThirdPerson/Blueprints/BP_Player_Character.QuestLogComponent_BP` (`/Game/Blueprints/Common_BPFL.GetMyPlayerCharacter`)) "10001"))))