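; Quest location marker actor that completes an objective when BP_Player_Character overlaps it.
; The fertilize-soil location requires a fertilizer item in the player's inventory; other locations complete unconditionally.
; The compost-bin apple check falls through to that fertilizer branch when empty, so it completes without apples too.
; Completion reports its ObjectiveID to the player, then destroys the marker after a short delay.
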(event `self.ReceiveActorBeginOverlap`
  (params (OtherActor :type "Actor Object Reference"))
  (bind _asbp_player_character (cast `/Game/ThirdPerson/Blueprints/BP_Player_Character` OtherActor))
  (if (`KismetTextLibrary.EqualEqual_TextText` (`self.LocationName`) (`self.compostbinlocation`))
    (bind (_item _success _quantity) (`/Game/ThirdPerson/Blueprints/BP_Player_Character.GetItem` _asbp_player_character "/Game/Blueprints/Inventory/BP_AppleItem.BP_AppleItem_C"))
    (if (> _quantity 0)
      (`/Game/ThirdPerson/Blueprints/BP_Player_Character.OnObjectiveIDCalled` _asbp_player_character (`self.ObjectiveID`) 1 :!label _label)
      (`KismetSystemLibrary.Delay` 1.0)
      (`self.K2_DestroyActor`)
      (else
        (if (`KismetTextLibrary.EqualEqual_TextText` (`self.LocationName`) (`self.FertilizeSoilLocation`)) :!label _label_2
          (bind (_item_2 _success_2 _quantity_2) (`/Game/ThirdPerson/Blueprints/BP_Player_Character.GetItem` _asbp_player_character "/Game/Blueprints/Inventory/BP_FertilizerItem.BP_FertilizerItem_C"))
          (if (> _quantity_2 0)
            (goto _label))
          (else
            (goto _label)))))
    (else
      (goto _label_2))))

(fn `UserConstructionScript`)