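; Base quest actor that tracks one quest's staged objectives, loaded from a data table by QuestID.
; It listens for the player's objective-ID events and seeds one objective type from inventory on BeginPlay, counting progress in a per-objective map.
; Completed objectives add a HUD notification; finished stages load the next, and the last marks the quest completed, turning it in through the player's quest log if AutoComplete is set.
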(event `self.ReceiveBeginPlay`
  (`self.GetQuestDetails`)
  (add `/Game/ThirdPerson/Blueprints/BP_Player_Character.OnObjectiveIDCalled` (`/Game/Blueprints/Common_BPFL.GetMyPlayerCharacter`) (`|CreateDelegate` :!event `On Objective IDHeard`))
  (for _array_element (`.Objectives_22_E0ECAC674113154B8263C391F91EB90D` (break `/Game/Blueprints/QuestSystem/SStageDetails` (`self.CurrentStageDetails`)))
    (bind ((`Type_19_D0EF20374852E91B1A91E58D97636BA8` _type) (`ObjectiveID_9_B83323D3490BAB82E0AA39BF84A0344A` _objectiveid)) (break `/Game/Blueprints/QuestSystem/SObjectiveDetails` _array_element))
    (if (`|EnumEquality` _type "NewEnumerator2")
      (bind _value (`/Game/ThirdPerson/Blueprints/BP_Player_Character.Query Inventory` (`/Game/Blueprints/Common_BPFL.GetMyPlayerCharacter`) (`KismetStringLibrary.Conv_StringToName` _objectiveid)))
      (`self.On Objective IDHeard` _objectiveid _value)))
  (`KismetSystemLibrary.Delay` 1.0)
  (bind _local_allcomplete1 (`self.IsAllObjectivesComplete`))
  (set `self.IsCompleted` _local_allcomplete1))

(fn `GetObjectiveDataByID`
  (params (ObjectiveID :type String))
  (returns (`Array Element` :type "/Game/Blueprints/QuestSystem/SObjectiveDetails Structure"))
  (for _array_element (`.Objectives_22_E0ECAC674113154B8263C391F91EB90D` (break `/Game/Blueprints/QuestSystem/SStageDetails` (`self.CurrentStageDetails`)))
    (if (`KismetStringLibrary.EqualEqual_StrStr` (`.ObjectiveID_9_B83323D3490BAB82E0AA39BF84A0344A` (break `/Game/Blueprints/QuestSystem/SObjectiveDetails` _array_element)) ObjectiveID)
      (return _array_element))))

(fn `GetQuestDetails`
  (locals (NewLocalVar :type "/Game/Blueprints/QuestSystem/SQuestDetails Structure"))
  (bind _returnvalue (`|GetDataTableRow` "/Game/Blueprints/QuestSystem/QuestData.QuestData" (`self.QuestID`))
    (:`then`
      (bind _output_get (set `self.QuestDetails` _returnvalue))
      (bind _output_get_2 (set `self.CurrentStageDetails` (`|GetArrayItem` (`.Stages_17_D8A614CF4E673C6EC6849FBF8A66D946` (break `/Game/Blueprints/QuestSystem/SQuestDetails` _output_get)) (`self.CurrentStage`))))
      (`BlueprintMapLibrary.Map_Clear` (`self.CurrentObjectiveProgress`))
      (for _array_element (`.Objectives_22_E0ECAC674113154B8263C391F91EB90D` (break `/Game/Blueprints/QuestSystem/SStageDetails` _output_get_2))
        (`BlueprintMapLibrary.Map_Add` (`self.CurrentObjectiveProgress`) (`.ObjectiveID_9_B83323D3490BAB82E0AA39BF84A0344A` (break `/Game/Blueprints/QuestSystem/SObjectiveDetails` _array_element)))))))

(fn `IsAllObjectivesComplete`
  (returns (Local_AllComplete1 :type Boolean))
  (locals (Local_AllComplete :type Boolean :default true))
  (for _array_element (`.Objectives_22_E0ECAC674113154B8263C391F91EB90D` (break `/Game/Blueprints/QuestSystem/SStageDetails` (`self.CurrentStageDetails`)))
    (bind (_objectivename _description _type _objectiveid) (break `/Game/Blueprints/QuestSystem/SObjectiveDetails` _array_element))
    (if (not (>= (`BlueprintMapLibrary.Map_Find` (`self.CurrentObjectiveProgress`) _objectiveid) (`.Quantity_12_8A4077D943D53B90E031A9BB540F9302` (break `/Game/Blueprints/QuestSystem/SObjectiveDetails` (`self.GetObjectiveDataByID` _objectiveid)))))
      (bind _output_get (set `local.Local_AllComplete` false))
      (return _output_get)))
  (return (`local.Local_AllComplete`)))

(fn `IsObjectiveComplete`
  (params (ObjectiveID :type String))
  (bind (_questdetails_questname _questdetails_logdescription _questdetails_trackerdescription _questdetails_ismain _questdetails_stages) (break `/Game/Blueprints/QuestSystem/SQuestDetails` (`self.QuestDetails`)))
  (bind (_questdetails_questname_2 _questdetails_logdescription_2 _questdetails_trackerdescription_2 _questdetails_ismain_2 _questdetails_stages_2 _questdetails_autoaccept _questdetails_autocomplete) (break `/Game/Blueprints/QuestSystem/SQuestDetails` (`self.QuestDetails`)))
  (bind ((`ObjectiveName_2_1ADBD56445F8400D76AB6FA7CC6B0B5A` _objectivename) (`Description_4_0BA9599E49ACA3094E650AA91933DEF0` _description) (`Quantity_12_8A4077D943D53B90E031A9BB540F9302` _quantity)) (break `/Game/Blueprints/QuestSystem/SObjectiveDetails` (`self.GetObjectiveDataByID` ObjectiveID)))
  (if (>= (`BlueprintMapLibrary.Map_Find` (`self.CurrentObjectiveProgress`) (`local.ObjectiveID`)) _quantity)
    (bind _foundwidgets (`WidgetBlueprintLibrary.GetAllWidgetsOfClass` "/Game/ThirdPerson/HUD/WBP_HUD.WBP_HUD_C"))
    (bind _returnvalue (`|CreateWidget` "/Game/Blueprints/QuestSystem/QuestUI/WBP_QuestNotification.WBP_QuestNotification_C" null _objectivename))
    (`VerticalBox.AddChildToVerticalBox` (`/Game/ThirdPerson/HUD/WBP_HUD.BOX_Notifications` (`|GetArrayItem` _foundwidgets)) _returnvalue)
    (bind _local_allcomplete1 (`self.IsAllObjectivesComplete`))
    (if _local_allcomplete1
      (bind _result (`/Engine/EditorBlueprintResources/StandardMacros.IncrementInt` (`self.CurrentStage`))
        (:`  `
          (if (`KismetArrayLibrary.Array_IsValidIndex` _questdetails_stages _result)
            (`self.GetQuestDetails`)
            (else
              (set `self.IsCompleted` true)
              (if _questdetails_autocomplete
                (`/Game/Blueprints/QuestSystem/QuestLogComponent_BP.TurnInQuest` (`self.GetComponentByClass` (`GameplayStatics.GetPlayerCharacter` 0) "/Game/Blueprints/QuestSystem/QuestLogComponent_BP.QuestLogComponent_BP_C") (`self.QuestID`))))))))))

(fn `On Objective IDHeard`
  (params (ObjectiveID :type String) (Value :type Integer :default 1))
  (bind (_value _returnvalue) (`BlueprintMapLibrary.Map_Find` (`self.CurrentObjectiveProgress`) (`local.ObjectiveID`)))
  (if (> (`KismetMathLibrary.SignOfInteger` Value) 0)
    (if _returnvalue
      (if (< _value (`.Quantity_12_8A4077D943D53B90E031A9BB540F9302` (break `/Game/Blueprints/QuestSystem/SObjectiveDetails` (`self.GetObjectiveDataByID` (`local.ObjectiveID`)))))
        (`BlueprintMapLibrary.Map_Add` (`self.CurrentObjectiveProgress`) (`local.ObjectiveID`) (+ _value (`local.Value`)))
        (`self.IsObjectiveComplete` (`local.ObjectiveID`))
        (`self.OnObjectiveHeard`)
        (return))
      (else
        (return)))))

(fn `UserConstructionScript`)