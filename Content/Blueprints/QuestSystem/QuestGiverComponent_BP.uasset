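; Quest giver component that lets its owning actor offer a data table quest and handle its reward turn-in.
; InteractWith checks the player's quest log, then either auto-accepts a new quest or shows the quest offer widget.
; For a known quest that is completed but not turned in, it shows the rewards widget instead.
; Each handled interaction returns the owner's display name, and both widgets receive the quest row and ID.
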(fn `DisplayQuest`
  (bind (_questdata_datatable _questdata_rowname) (break `DataTableRowHandle` (`self.QuestData`)))
  (bind _returnvalue (`|GetDataTableRow` _questdata_datatable _questdata_rowname)
    (:`then`
      (bind _returnvalue_2 (`|CreateWidget` "/Game/Blueprints/QuestSystem/QuestUI/WBP_QuestGiver.WBP_QuestGiver_C" null _returnvalue _questdata_rowname))
      (`UserWidget.AddToViewport` _returnvalue_2 0))))

(fn `DisplayRewards`
  (bind (_questdata_datatable _questdata_rowname) (break `DataTableRowHandle` (`self.QuestData`)))
  (bind _returnvalue (`|GetDataTableRow` "/Game/Blueprints/QuestSystem/QuestData.QuestData" _questdata_rowname)
    (:`then`
      (bind _returnvalue_2 (`|CreateWidget` "/Game/Blueprints/QuestSystem/QuestUI/WBP_QuestRewards.WBP_QuestRewards_C" null _returnvalue _questdata_rowname))
      (`UserWidget.AddToViewport` _returnvalue_2 0))))

(fn `InteractWith`
  (returns (ObjectiveID :type String))
  (bind (_questdata_datatable _questdata_rowname) (break `DataTableRowHandle` (`self.QuestData`)))
  (bind (_questdata_datatable_2 _questdata_rowname_2) (break `DataTableRowHandle` (`self.QuestData`)))
  (bind (_questdata_datatable_3 _questdata_rowname_3) (break `DataTableRowHandle` (`self.QuestData`)))
  (bind (_questdata_datatable_4 _questdata_rowname_4) (break `DataTableRowHandle` (`self.QuestData`)))
  (bind _returnvalue (`KismetSystemLibrary.GetDisplayName` (`self.GetOwner`)))
  (bind _returnvalue_2 (`Actor.GetComponentByClass` (`/Game/Blueprints/Common_BPFL.GetMyPlayerCharacter`) "/Game/Blueprints/QuestSystem/QuestLogComponent_BP.QuestLogComponent_BP_C"))
  (bind _questlogcomponent_bp (`/Game/ThirdPerson/Blueprints/BP_Player_Character.QuestLogComponent_BP` (`/Game/Blueprints/Common_BPFL.GetMyPlayerCharacter`)))
  (if (and (not (`/Game/Blueprints/QuestSystem/QuestLogComponent_BP.QueryCompletedQuest` _questlogcomponent_bp _questdata_rowname)) (not (`/Game/Blueprints/QuestSystem/QuestLogComponent_BP.QueryActiveQuest` _questlogcomponent_bp _questdata_rowname)))
    (bind _returnvalue_3 (`|GetDataTableRow` "/Game/Blueprints/QuestSystem/QuestData.QuestData" _questdata_rowname_3)
      (:`then`
        (if (`.AutoAccept_19_D1547D00472108DA3B72B29682A09591` (break `/Game/Blueprints/QuestSystem/SQuestDetails` _returnvalue_3))
          (`/Engine/EditorBlueprintResources/StandardMacros.IsValid` _returnvalue_2
            (:`Is Valid`
              (`/Game/Blueprints/QuestSystem/QuestLogComponent_BP.AddNewQuest` _returnvalue_2 _questdata_rowname_4)
              (return (`KismetSystemLibrary.GetDisplayName` (`self.GetOwner`)))))
          (else
            (`self.DisplayQuest`)
            (return _returnvalue)))))
    (else
      (bind _array_element (`/Game/Blueprints/QuestSystem/QuestLogComponent_BP.GetQuestActor` (`/Game/ThirdPerson/Blueprints/BP_Player_Character.QuestLogComponent_BP` (`/Game/Blueprints/Common_BPFL.GetMyPlayerCharacter`)) _questdata_rowname_2))
      (if (and (`/Game/Blueprints/QuestSystem/QuestBase_BP.IsCompleted` _array_element) (not (`/Game/Blueprints/QuestSystem/QuestBase_BP.IsTurnedIn` _array_element)))
        (`self.DisplayRewards`)
        (return _returnvalue)))))