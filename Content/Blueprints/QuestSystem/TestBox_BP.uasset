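; TestBox_BP is a test interactable box for the quest system that reports an objective ID when the player interacts with it.
; Its Box overlap events toggle NextToInteractable on BP_Player_Character, and entering also clears DoesTakeEnergy.
; Interact passes ObjectiveID to the player's CallOnObjectiveIDCalled and prints it for debugging.
; InteractWith returns a fixed name string identifying the box.
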(event `self.Box.OnComponentBeginOverlap`
  (params (OverlappedComponent :type "PrimitiveComponent Object Reference") (OtherActor :type "Actor Object Reference") (OtherComp :type "PrimitiveComponent Object Reference") (OtherBodyIndex :type Integer) (bFromSweep :type Boolean) (SweepResult :type "HitResult Structure (by ref)"))
  (bind _asbp_player_character (cast `/Game/ThirdPerson/Blueprints/BP_Player_Character` OtherActor))
  (set `/Game/ThirdPerson/Blueprints/BP_Player_Character.NextToInteractable` true _asbp_player_character)
  (set `/Game/ThirdPerson/Blueprints/BP_Player_Character.DoesTakeEnergy` false _asbp_player_character))

(event `self.Box.OnComponentEndOverlap`
  (params (OverlappedComponent :type "PrimitiveComponent Object Reference") (OtherActor :type "Actor Object Reference") (OtherComp :type "PrimitiveComponent Object Reference") (OtherBodyIndex :type Integer))
  (bind _asbp_player_character (cast `/Game/ThirdPerson/Blueprints/BP_Player_Character` OtherActor))
  (set `/Game/ThirdPerson/Blueprints/BP_Player_Character.NextToInteractable` false _asbp_player_character))

(event `/Game/Blueprints/Interact_BPI.Interact`
  (params (`Player Character` :type "/Game/ThirdPerson/Blueprints/BP_Player_Character Object Reference"))
  (bind _objectiveid (`self.ObjectiveID`))
  (`/Game/ThirdPerson/Blueprints/BP_Player_Character.OnObjectiveIDCalled` `Player Character` _objectiveid)
  (`KismetSystemLibrary.PrintString` (`KismetStringLibrary.Concat_StrStr` "The Box: " _objectiveid)))

(fn `InteractWith`
  (returns (ObjectiveID :type String))
  (return "thebox"))

(fn `UserConstructionScript`)