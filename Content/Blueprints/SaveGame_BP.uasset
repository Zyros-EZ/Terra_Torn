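; SaveGame Blueprint that stores player and quest state and restores it on load.
; Player inventory, energy and gold are copied to and from the character.
; The quest log's active and completed lists are saved, while each quest's stage and objective progress go into a map keyed by quest ID.
; Loading re-adds each active quest to the quest log component, applies its mapped progress, then restores both lists.
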(fn `LoadPlayerVariables`
  (params (PlayerCharacter :type "/Game/ThirdPerson/Blueprints/BP_Player_Character Object Reference"))
  (set `/Game/ThirdPerson/Blueprints/BP_Player_Character.Inventory` (`self.Inventory`) PlayerCharacter)
  (set `/Game/ThirdPerson/Blueprints/BP_Player_Character.Energy` (`self.PlayerEnergy`) PlayerCharacter)
  (set `/Game/ThirdPerson/Blueprints/BP_Player_Character.PlayerGold` (`self.PlayerGold`) PlayerCharacter))

(fn `LoadQuests`
  (params (QuestLogComponent :type "/Game/Blueprints/QuestSystem/QuestLogComponent_BP Object Reference"))
  (for _array_element (`self.CurrentActiveQuests`)
    (bind _returnvalue (`/Game/Blueprints/QuestSystem/QuestLogComponent_BP.AddNewQuest` QuestLogComponent _array_element))
    (bind (_progress _currrentstage) (break `/Game/Blueprints/QuestSystem/SQuestSaveData` (`BlueprintMapLibrary.Map_Find` (`self.QuestProgress`) _array_element)))
    (set `/Game/Blueprints/QuestSystem/QuestBase_BP.CurrentStage` _currrentstage _returnvalue)
    (set `/Game/Blueprints/QuestSystem/QuestBase_BP.CurrentObjectiveProgress` _progress _returnvalue))
  (set `/Game/Blueprints/QuestSystem/QuestLogComponent_BP.CurrentActiveQuests` (`self.CurrentActiveQuests`) QuestLogComponent)
  (set `/Game/Blueprints/QuestSystem/QuestLogComponent_BP.CompletedQuests` (`self.CompletedQuests`) QuestLogComponent))

(fn `SavePlayerVariables`
  (params (PlayerCharacter :type "/Game/ThirdPerson/Blueprints/BP_Player_Character Object Reference"))
  (set `self.Inventory` (`/Game/ThirdPerson/Blueprints/BP_Player_Character.Inventory` PlayerCharacter))
  (set `self.PlayerEnergy` (`/Game/ThirdPerson/Blueprints/BP_Player_Character.Energy` PlayerCharacter))
  (set `self.PlayerGold` (`/Game/ThirdPerson/Blueprints/BP_Player_Character.PlayerGold` PlayerCharacter)))

(fn `SaveQuestDetails`
  (params (Quest :type "/Game/Blueprints/QuestSystem/QuestBase_BP Object Reference"))
  (`BlueprintMapLibrary.Map_Add` (`self.QuestProgress`) (`/Game/Blueprints/QuestSystem/QuestBase_BP.QuestID` Quest) (make `/Game/Blueprints/QuestSystem/SQuestSaveData` (`/Game/Blueprints/QuestSystem/QuestBase_BP.CurrentObjectiveProgress` Quest) (`/Game/Blueprints/QuestSystem/QuestBase_BP.CurrentStage` Quest))))

(fn `SaveQuestLog`
  (params (QuestLog :type "/Game/Blueprints/QuestSystem/QuestLogComponent_BP Object Reference"))
  (set `self.CurrentActiveQuests` (`/Game/Blueprints/QuestSystem/QuestLogComponent_BP.CurrentActiveQuests` QuestLog))
  (set `self.CompletedQuests` (`/Game/Blueprints/QuestSystem/QuestLogComponent_BP.CompletedQuests` QuestLog)))