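; Base spline actor that tiles a chosen static mesh along its spline as deforming spline mesh components, built in the Construction Script.
; Section length optionally derives from actor scale on the forward axis, and sets the segment count, with MustBeFullLengthMeshes dropping the final partial segment.
; Helper functions sample each segment's local start and end by distance, clamping tangents to section length to match the segment.
; Each segment receives the configured forward axis and collision type.
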(fn `Get End Position`
  (params (Index :type Integer))
  (returns (Position :type "Vector Structure") (Tangent :type "Vector Structure"))
  (bind _spline (`self.Spline`))
  (bind _returnvalue (* (+ Index 1) (`self.SectionLength`)))
  (return (`SplineComponent.GetLocationAtDistanceAlongSpline` _spline _returnvalue "Local") (`KismetMathLibrary.ClampVectorSize` (`SplineComponent.GetTangentAtDistanceAlongSpline` _spline _returnvalue "Local") 0.0 (`self.SectionLength`))))

(fn `Get Start Position`
  (params (index :type Integer))
  (returns (Position :type "Vector Structure") (Tangent :type "Vector Structure"))
  (bind _spline (`self.Spline`))
  (bind _returnvalue (* index (`self.SectionLength`)))
  (return (`SplineComponent.GetLocationAtDistanceAlongSpline` _spline _returnvalue "Local") (`KismetMathLibrary.ClampVectorSize` (`SplineComponent.GetTangentAtDistanceAlongSpline` _spline _returnvalue "Local") 0.0 (`self.SectionLength`))))

(fn `UserConstructionScript`
  (locals (`Loop Index` :type Integer) (VectorValue :type "Float (double-precision)"))
  (if (`self.AllowScaling`)
    ;[1 1 1] Scale the Spline
    (switch `ESplineMeshAxis` (`self.ForwardAxis`)
      (:`X`
        (set `local.VectorValue` (.x (`self.GetActorScale3D`))))
      (:`Y`
        (set `local.VectorValue` (.y (`self.GetActorScale3D`))))
      (:`Z`
        (set `local.VectorValue` (.z (`self.GetActorScale3D`)))))
    (set `self.SectionLength` (* (`local.VectorValue`) 100.0)))
  (if (`self.MustBeFullLengthMeshes`)
    ;[1 1 1] Full length meshes
    (for _index (range (`KismetMathLibrary.FTrunc` (/ (`SplineComponent.GetSplineLength` (`self.Spline`)) (`self.SectionLength`))))
      (set `local.Loop Index` _index)
      (bind _returnvalue (`AddComponent|NODE_AddSplineMeshComponent-0` :!label _label))
      (`StaticMeshComponent.SetStaticMesh` _returnvalue (`self.SplineMesh`))
      (`SplineMeshComponent.SetForwardAxis` _returnvalue (`self.ForwardAxis`) true)
      (bind (_position _tangent) (`self.Get Start Position` (`local.Loop Index`)))
      (bind (_position_2 _tangent_2) (`self.Get End Position` (`local.Loop Index`)))
      (`SplineMeshComponent.SetStartAndEnd` _returnvalue _position _tangent _position_2 _tangent_2 true)
      (`PrimitiveComponent.SetCollisionEnabled` _returnvalue (`self.CollisionType`)))
    (else
      ;[1 1 1] Determine Spline Mesh Count
      (for _index_2 (range (+ (`KismetMathLibrary.FTrunc` (/ (`SplineComponent.GetSplineLength` (`self.Spline`)) (`self.SectionLength`))) 1))
        (set `local.Loop Index` _index_2)
        (goto _label)))))