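; Interactable soil plot that the player fertilizes to prepare it for planting kiwi seeds.
; Box overlap shows or hides the interact prompt and flags the player as near an interactable.
; Interacting spends fertilizer and energy through FertilizerCheck, then swaps to dirt material, plays a hoe sound, reports objective progress and spawns a location marker.
; The seed menu fed by SeedCheck inventory counts is disconnected, so fertilized soil only looks up a crop actor.
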(event `self.ReceiveActorBeginOverlap`
  (params (OtherActor :type "Actor Object Reference")))

(event `self.ReceiveBeginPlay`
  (`|ExecutionSequence`
    (:`then_0`
      (bind _returnvalue (`|CreateWidget` "/Game/P_Interact.P_Interact_C"))
      (set `self.Interact prompt` _returnvalue))
    (:`then_1`
      (bind _returnvalue_2 (`|CreateWidget` "/Game/Blueprints/Crops/WBP_PlantSeed.WBP_PlantSeed_C"))
      (set `self.SeedUI` _returnvalue_2))
    (:`then_2`
      (set `self.Location` (`SceneComponent.K2_GetComponentLocation` (`self.StaticMeshComponent`))))))

(event `/Game/Blueprints/Interact_BPI.Interact`
  (params (`Player Character` :type "/Game/ThirdPerson/Blueprints/BP_Player_Character Object Reference"))
  ;[1 1 1] Interaction - Fertilize Soil/Open UI
  (set `self.PlayerCharacter` `Player Character`)
  (if (not (`self.IsFertilized`))
    (`self.FertilizeSoil`)
    (else
      (bind _returnvalue (`GameplayStatics.GetActorOfClass` "/Game/Blueprints/Crops/ParentCrop_BP.ParentCrop_BP_C")))))

(event `self.Box.OnComponentBeginOverlap`
  (params (OverlappedComponent :type "PrimitiveComponent Object Reference") (OtherActor :type "Actor Object Reference") (OtherComp :type "PrimitiveComponent Object Reference") (OtherBodyIndex :type Integer) (bFromSweep :type Boolean) (SweepResult :type "HitResult Structure (by ref)"))
  ;[1 1 1] Interact Action and Text
  (if (== OtherActor (`GameplayStatics.GetPlayerCharacter` 0))
    (`UserWidget.AddToViewport` (`self.Interact prompt`) 0)
    (set `/Game/ThirdPerson/Blueprints/BP_Player_Character.NextToInteractable` true (`/Game/Blueprints/Common_BPFL.GetMyPlayerCharacter`))))

(event `self.Box.OnComponentEndOverlap`
  (params (OverlappedComponent :type "PrimitiveComponent Object Reference") (OtherActor :type "Actor Object Reference") (OtherComp :type "PrimitiveComponent Object Reference") (OtherBodyIndex :type Integer))
  ;[1 1 1] Interact Action and Text
  (if (== (`GameplayStatics.GetPlayerCharacter` 0) OtherActor)
    (`Widget.RemoveFromParent` (`self.Interact prompt`))
    (if (`self.UIOpen`)
      (`Widget.RemoveFromParent` (`self.SeedUI`))
      (set `self.UIOpen` false))))

(fn `FertilizerCheck`
  (returns (HasFertilizer :type Boolean))
  (bind _hasitem (`/Game/Blueprints/Inventory/Inventory.HasItemInInventory` (`/Game/ThirdPerson/Blueprints/BP_Player_Character.NewInventory` (`self.PlayerCharacter`)) "NewEnumerator10"))
  (if _hasitem
    (`/Game/Blueprints/Interact_BPI.TakePlayerEnergy` (`self.PlayerCharacter`) true)
    (`/Game/Blueprints/Inventory/Inventory.Consume From Inventory` (`/Game/ThirdPerson/Blueprints/BP_Player_Character.NewInventory` (`self.PlayerCharacter`)) "NewEnumerator10" 1)
    (return _hasitem)
    (else
      (set `self.IsFertilized` false)
      (return false))))

(fn `FertilizeSoil`
  (bind _hasfertilizer (`self.FertilizerCheck`))
  (if _hasfertilizer
    (`GameplayStatics.SpawnSoundAtLocation` "/Game/SFX/Hoe.Hoe" (`self.Location`) (struct) 1.0 1.0 0.0 null null)
    (`PrimitiveComponent.SetMaterial` (`self.StaticMeshComponent`) 0 "/Game/Materials/M_Dirt.M_Dirt")
    (set `self.IsFertilized` true)
    (set `/Game/ThirdPerson/Blueprints/BP_Player_Character.DoesTakeEnergy` false (`self.PlayerCharacter`))
    (bind _output_get (set `self.FertilizeObjectiveQuantity` (+ (`self.FertilizeObjectiveQuantity`) 1)))
    (`/Game/ThirdPerson/Blueprints/BP_Player_Character.OnObjectiveIDCalled` (`self.PlayerCharacter`) "fertilizesoil" _output_get)
    (`|SpawnActorFromClass` "/Game/Blueprints/QuestSystem/LocationMarker_BP.LocationMarker_BP_C" (`KismetMathLibrary.MakeTransform` (`self.Location`) (struct) (5.0 5.0 1.0)) "Undefined" "MultiplyWithRoot" null (`self.LocationName`) (`self.ObjectiveID`) null)))

(fn `InteractWith`
  (returns (ObjectiveID :type String))
  (return ""))

(fn `SeedCheck`
  (returns (SmallKiwiAmount :type Integer) (BigKiwiAmount :type Integer) (MetalKiwiAmount :type Integer) (IceyKiwiAmount :type Integer) (HeatedKiwiAmount :type Integer))
  (bind _newinventory (`/Game/ThirdPerson/Blueprints/BP_Player_Character.NewInventory` (`self.PlayerCharacter`)))
  (`|ExecutionSequence`
    (:`then_0`
      (bind _count (`/Game/Blueprints/Inventory/Inventory.GetInventoryCount` _newinventory "NewEnumerator5")))
    (:`then_1`
      (bind _count_2 (`/Game/Blueprints/Inventory/Inventory.GetInventoryCount` _newinventory "NewEnumerator6")))
    (:`then_2`
      (bind _count_3 (`/Game/Blueprints/Inventory/Inventory.GetInventoryCount` _newinventory "NewEnumerator7")))
    (:`then_3`
      (bind _count_4 (`/Game/Blueprints/Inventory/Inventory.GetInventoryCount` _newinventory "NewEnumerator8")))
    (:`then_4`
      (bind _count_5 (`/Game/Blueprints/Inventory/Inventory.GetInventoryCount` _newinventory "NewEnumerator3"))))
  (return _count _count_2 _count_3 _count_4 _count_5))

(fn `TakePlayerEnergy`
  (params (isHarvestable :type Boolean))
  (returns (HasEnergy :type Boolean))
  (return false))

(fn `UserConstructionScript`)